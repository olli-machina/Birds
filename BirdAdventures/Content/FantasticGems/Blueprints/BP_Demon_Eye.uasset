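; Configurable Demon Eye gemstone prop from FantasticGems, built entirely in the Construction Script with no active runtime logic.
; A shape option can flatten the Gemstone mesh into a pebble, then a Freestyle-or-Preset switch drives a dynamic material instance.
; Freestyle sets colors, toggleable internal effects like fire, cracks, cloud and eye, plus a randomized Time parameter.
; Presets swap among ten static meshes and override only life and hue.
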(event EventBeginPlay)

(event Collision|EventActorBeginOverlap
  (params (OtherActor :type Actor%20Object%20Reference)))

(event EventTick
  (params (DeltaSeconds :type Float%20%28single-precision%29)))

(fn ConstructionScript
  (bind _gemstone (Variables|Default|GetGemstone))
  (bind _gemstone_2 (Variables|Default|GetGemstone))
  (bind _gemstone_3 (Variables|Default|GetGemstone))
  (switch Utilities|FlowControl|Switch|SwitchonENUM_Demon_Eye_002 (Variables|Control|GetPick%20Shape)
    (:NewEnumerator0
      _)
    (:NewEnumerator1
      (Transformation|SetRelativeScale3D (Variables|Default|GetGemstone) "1.000000,1.000000,0.700000")))
  (switch Utilities|FlowControl|Switch|SwitchonENUM_Demon_Eye_001 (Variables|Control|GetFreestyle%20or%20Preset)
    (:NewEnumerator0
      (bind _returnvalue (Rendering|Material|CreateDynamicMaterialInstance _gemstone_2 0 (Rendering|Material|GetMaterial _gemstone_2 0) :!class /Script/Engine.PrimitiveComponent))
      (Rendering|Material|SetScalarParameterValue _returnvalue "Has Life" (Variables|Life|GetGemstone%20Life) :!class /Script/Engine.MaterialInstanceDynamic)
      (Rendering|Material|SetScalarParameterValue _returnvalue "Albedo Hue" (Variables|Color|GetAlbedo%20Hue) :!class /Script/Engine.MaterialInstanceDynamic)
      (Rendering|Material|SetScalarParameterValue _returnvalue "Hue" (Variables|Color|GetHue) :!class /Script/Engine.MaterialInstanceDynamic)
      (Rendering|Material|SetVectorParameterValue _returnvalue "Color Multiplier" (Variables|Color|GetMultiply%20Color) :!class /Script/Engine.MaterialInstanceDynamic)
      (Rendering|Material|SetVectorParameterValue _returnvalue "Color Add" (Variables|Color|GetAdd%20Color) :!class /Script/Engine.MaterialInstanceDynamic)
      (Rendering|Material|SetVectorParameterValue _returnvalue "Color within" (Variables|Color|GetColor%20Within) :!class /Script/Engine.MaterialInstanceDynamic)
      (Rendering|Material|SetVectorParameterValue _returnvalue "Subsurface Color Add" (Variables|Color|GetSubsurface%20Color%20Tweak) :!class /Script/Engine.MaterialInstanceDynamic)
      (Rendering|Material|SetVectorParameterValue _returnvalue "Cracks Color" (Variables|Color|GetCracks%20Color) :!class /Script/Engine.MaterialInstanceDynamic)
      (if (Variables|Features|GetLife)
        (Variables|Default|SetHas%20Life 1.0)
        (else
          (Variables|Default|SetHas%20Life 0.0)))
      (if (Variables|Features|GetInternal%20Fire)
        (Variables|Default|SetFire%20Within%20Intensity 1.0)
        (else
          (Variables|Default|SetFire%20Within%20Intensity 0.0)))
      (if (Variables|Features|GetInternal%20Pulse)
        (Variables|Default|SetAdd%20Internal%20Pulse 1.0)
        (else
          (Variables|Default|SetAdd%20Internal%20Pulse 0.0)))
      (if (Variables|Features|GetInternal%20Craks)
        (Variables|Default|SetAdd%20Internal%20Craks 1.0)
        (else
          (Variables|Default|SetAdd%20Internal%20Craks 0.0)))
      (if (Variables|Features|GetInternal%20Cloud)
        (Variables|Default|SetAdd%20Internal%20Cloud 1.0)
        (else
          (Variables|Default|SetAdd%20Internal%20Cloud 0.0)))
      (if (Variables|Features|GetInternal%20Cloud%20Motion)
        (Variables|Default|SetAdd%20Internal%20Cloud%20Motion 1.0)
        (else
          (Variables|Default|SetAdd%20Internal%20Cloud%20Motion 0.0)))
      (if (Variables|Features|GetInternal%20Gradient)
        (Variables|Default|SetAdd%20Internal%20Gradient 1.0)
        (else
          (Variables|Default|SetAdd%20Internal%20Gradient 0.0)))
      (if (Variables|Features|GetInternal%20Eye)
        (Variables|Default|SetAdd%20Internal%20Dot 1.0)
        (else
          (Variables|Default|SetAdd%20Internal%20Dot 0.0)))
      (Rendering|Material|SetScalarParameterValue _returnvalue "Fire Within Intensity" (Variables|Default|GetFire%20Within%20Intensity) :!class /Script/Engine.MaterialInstanceDynamic)
      (Rendering|Material|SetScalarParameterValue _returnvalue "Add Internal Pulse" (Variables|Default|GetAdd%20Internal%20Pulse) :!class /Script/Engine.MaterialInstanceDynamic)
      (Rendering|Material|SetScalarParameterValue _returnvalue "Add Internal Craks" (Variables|Default|GetAdd%20Internal%20Craks) :!class /Script/Engine.MaterialInstanceDynamic)
      (Rendering|Material|SetScalarParameterValue _returnvalue "Add Internal Cloud" (Variables|Default|GetAdd%20Internal%20Cloud) :!class /Script/Engine.MaterialInstanceDynamic)
      (Rendering|Material|SetScalarParameterValue _returnvalue "Add Internal Cloud Motion" (Variables|Default|GetAdd%20Internal%20Cloud%20Motion) :!class /Script/Engine.MaterialInstanceDynamic)
      (Rendering|Material|SetScalarParameterValue _returnvalue "Add Internal Gradient" (Variables|Default|GetAdd%20Internal%20Gradient) :!class /Script/Engine.MaterialInstanceDynamic)
      (Rendering|Material|SetScalarParameterValue _returnvalue "Add Internal Dot" (Variables|Default|GetAdd%20Internal%20Dot) :!class /Script/Engine.MaterialInstanceDynamic)
      (Rendering|Material|SetScalarParameterValue _returnvalue "Time" (Math|Random|RandomFloatinRange 0.4 1.1) :!class /Script/Engine.MaterialInstanceDynamic))
    (:NewEnumerator1
      (Components|StaticMesh|SetStaticMesh _gemstone_3 "/Game/FantasticGems/Meshes/SM_Demon_Eye_001.SM_Demon_Eye_001")
      (bind _returnvalue_2 (Rendering|Material|CreateDynamicMaterialInstance _gemstone 0 (Rendering|Material|GetMaterial _gemstone 0) :!class /Script/Engine.PrimitiveComponent :!label _label))
      (Rendering|Material|SetScalarParameterValue _returnvalue_2 "Has Life" (Variables|Life|GetGemstone%20Life) :!class /Script/Engine.MaterialInstanceDynamic)
      (Rendering|Material|SetScalarParameterValue _returnvalue_2 "Hue" (Variables|Color|GetHue) :!class /Script/Engine.MaterialInstanceDynamic))
    (:NewEnumerator2
      (Components|StaticMesh|SetStaticMesh _gemstone_3 "/Game/FantasticGems/Meshes/SM_Demon_Eye_002.SM_Demon_Eye_002")
      (goto _label))
    (:NewEnumerator3
      (Components|StaticMesh|SetStaticMesh _gemstone_3 "/Game/FantasticGems/Meshes/SM_Demon_Eye_003.SM_Demon_Eye_003")
      (goto _label))
    (:NewEnumerator4
      (Components|StaticMesh|SetStaticMesh _gemstone_3 "/Game/FantasticGems/Meshes/SM_Demon_Eye_004.SM_Demon_Eye_004")
      (goto _label))
    (:NewEnumerator5
      (Components|StaticMesh|SetStaticMesh _gemstone_3 "/Game/FantasticGems/Meshes/SM_Demon_Eye_005.SM_Demon_Eye_005")
      (goto _label))
    (:NewEnumerator6
      (Components|StaticMesh|SetStaticMesh _gemstone_3 "/Game/FantasticGems/Meshes/SM_Demon_Eye_006.SM_Demon_Eye_006")
      (goto _label))
    (:NewEnumerator7
      (Components|StaticMesh|SetStaticMesh _gemstone_3 "/Game/FantasticGems/Meshes/SM_Demon_Eye_007.SM_Demon_Eye_007")
      (goto _label))
    (:NewEnumerator8
      (Components|StaticMesh|SetStaticMesh _gemstone_3 "/Game/FantasticGems/Meshes/SM_Demon_Eye_008.SM_Demon_Eye_008")
      (goto _label))
    (:NewEnumerator9
      (Components|StaticMesh|SetStaticMesh _gemstone_3 "/Game/FantasticGems/Meshes/SM_Demon_Eye_009.SM_Demon_Eye_009")
      (goto _label))
    (:NewEnumerator10
      (Components|StaticMesh|SetStaticMesh _gemstone_3 "/Game/FantasticGems/Meshes/SM_Demon_Eye_010.SM_Demon_Eye_010")
      (goto _label))))