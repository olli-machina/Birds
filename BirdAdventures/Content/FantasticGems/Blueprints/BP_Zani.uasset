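; Configurable Zani gemstone Blueprint that builds its mesh and material entirely in the construction script, with no active event logic.
; The shape option swaps the mesh and clears normal and mask textures for all but Shard.
; Freestyle mode drives a dynamic MAT_Zani instance with selectable internal textures, bump offset and emissive settings; presets wrap MI_Zani instances with those shape textures.
; The custom FX texture is written to InternalColor, so it never reaches the FX parameter.
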(event EventBeginPlay)

(event Collision|EventActorBeginOverlap
  (params (OtherActor :type Actor%20Object%20Reference)))

(event EventTick
  (params (DeltaSeconds :type Float%20%28single-precision%29)))

(fn ConstructionScript
  (bind _gemstone (Variables|Default|GetGemstone))
  (bind _gemstone_2 (Variables|Default|GetGemstone))
  (bind _gemstone_3 (Variables|Default|GetGemstone))
  (switch Utilities|FlowControl|Switch|SwitchonENUM_Zani_001 (Variables|Control|GetSelect%20Shape)
    (:NewEnumerator0
      _)
    (:NewEnumerator1
      (Variables|Default|SetNormal 0)
      (Variables|Default|SetMasks 0)
      (Components|StaticMesh|SetStaticMesh _gemstone_3 "/Game/FantasticGems/Meshes/SM_Liquid_Metal_001.SM_Liquid_Metal_001"))
    (:NewEnumerator2
      (Variables|Default|SetNormal 0)
      (Variables|Default|SetMasks 0)
      (Components|StaticMesh|SetStaticMesh _gemstone_3 "/Game/FantasticGems/Meshes/SM_Demon_Eye_001.SM_Demon_Eye_001"))
    (:NewEnumerator3
      (Variables|Default|SetNormal 0)
      (Variables|Default|SetMasks 0)
      (Components|StaticMesh|SetStaticMesh _gemstone_3 "/Game/FantasticGems/Meshes/SM_Thunderstone_001.SM_Thunderstone_001")))
  (switch Utilities|FlowControl|Switch|SwitchonENUM_Demon_Eye_001 (Variables|Control|GetFreestyle%20or%20Preset)
    (:NewEnumerator0
      (bind _returnvalue (Rendering|Material|CreateDynamicMaterialInstance (Variables|Default|GetGemstone) 0 "/Game/FantasticGems/Materials/Master/MAT_Zani.MAT_Zani" :!class /Script/Engine.PrimitiveComponent))
      (Variables|Default|SetMaterial _returnvalue)
      (Rendering|Material|SetTextureParameterValue _returnvalue "Normal" (Variables|Default|GetNormal))
      (Rendering|Material|SetTextureParameterValue _returnvalue "Masks" (Variables|Default|GetMasks))
      (switch int (Variables|Internal|GetPick%20Internal%20Color%20Texture)
        (:1
          (Variables|Default|SetInternal%20Color "/Game/FantasticGems/Textures/T_Zani_001_C.T_Zani_001_C"))
        (:2
          (Variables|Default|SetInternal%20Color "/Game/FantasticGems/Textures/T_Zani_002_C.T_Zani_002_C"))
        (:3
          (Variables|Default|SetInternal%20Color "/Game/FantasticGems/Textures/T_Zani_003_C.T_Zani_003_C"))
        (:4
          (Variables|Default|SetInternal%20Color "/Game/FantasticGems/Textures/T_Zani_004_C.T_Zani_004_C"))
        (:5
          (Variables|Default|SetInternal%20Color "/Game/FantasticGems/Textures/T_Zani_005_C.T_Zani_005_C"))
        (:6
          (Variables|Default|SetInternal%20Color "/Game/FantasticGems/Textures/T_Zani_006_C.T_Zani_006_C"))
        (:7
          (Variables|Default|SetInternal%20Color "/Game/FantasticGems/Textures/T_Zani_007_C.T_Zani_007_C"))
        (:8
          (Variables|Default|SetInternal%20Color "/Game/FantasticGems/Textures/T_Zani_008_C.T_Zani_008_C"))
        (:9
          (Variables|Default|SetInternal%20Color "/Game/FantasticGems/Textures/T_Zani_009_C.T_Zani_009_C")))
      (if (Variables|Internal|GetUse%20Custom%20Internal%20Color%20Texture)
        (Variables|Default|SetInternal%20Color (Variables|Internal|GetCustom%20Internal%20Color%20Texture)))
      (Rendering|Material|SetTextureParameterValue _returnvalue "Internal Color" (Variables|Default|GetInternal%20Color))
      (switch int (Variables|Internal|GetPick%20Internal%20Color%20Texture)
        (:1
          (Variables|Default|SetFX "/Game/FantasticGems/Textures/T_Zani_001_M.T_Zani_001_M"))
        (:2
          (Variables|Default|SetFX "/Game/FantasticGems/Textures/T_Zani_002_M.T_Zani_002_M"))
        (:3
          (Variables|Default|SetFX "/Game/FantasticGems/Textures/T_Zani_003_M.T_Zani_003_M"))
        (:4
          (Variables|Default|SetFX "/Game/FantasticGems/Textures/T_Zani_004_M.T_Zani_004_M"))
        (:5
          (Variables|Default|SetFX "/Game/FantasticGems/Textures/T_Zani_005_M.T_Zani_005_M"))
        (:6
          (Variables|Default|SetFX "/Game/FantasticGems/Textures/T_Zani_004_M.T_Zani_004_M"))
        (:7
          (Variables|Default|SetFX "/Game/FantasticGems/Textures/T_Zani_007_M.T_Zani_007_M"))
        (:8
          (Variables|Default|SetFX "/Game/FantasticGems/Textures/T_Zani_007_M.T_Zani_007_M"))
        (:9
          (Variables|Default|SetFX "/Game/FantasticGems/Textures/T_Zani_009_M.T_Zani_009_M")))
      (if (Variables|Internal|GetUse%20Custom%20Internal%20Color%20Texture)
        (Variables|Default|SetInternal%20Color (Variables|Internal|GetCustom%20Internal%20FX%20Texture)))
      (Rendering|Material|SetTextureParameterValue _returnvalue "Internal FX" (Variables|Default|GetFX))
      (Rendering|Material|SetScalarParameterValue (Variables|Default|GetMaterial) "Internal Texture Size" (Variables|Internal|GetInternal%20Texture%20Size) :!class /Script/Engine.MaterialInstanceDynamic)
      (Rendering|Material|SetScalarParameterValue (Variables|Default|GetMaterial) "Reference Plane" (Variables|Internal|GetBump%20Offset%20Reference%20Plane) :!class /Script/Engine.MaterialInstanceDynamic)
      (Rendering|Material|SetScalarParameterValue (Variables|Default|GetMaterial) "Height Ratio" (Variables|Internal|GetBump%20Offset%20Height%20Ratio) :!class /Script/Engine.MaterialInstanceDynamic)
      (Rendering|Material|SetScalarParameterValue (Variables|Default|GetMaterial) "Emissive INtesnity" (Variables|Internal|GetEmissive%20Intesnity) :!class /Script/Engine.MaterialInstanceDynamic))
    (:NewEnumerator1
      (Rendering|Material|SetMaterial _gemstone 0 "/Game/FantasticGems/Materials/Instances/MI_Zani_001.MI_Zani_001")
      (bind _returnvalue_2 (Rendering|Material|CreateDynamicMaterialInstance _gemstone_2 0 (Rendering|Material|GetMaterial _gemstone_2 0) :!class /Script/Engine.PrimitiveComponent :!label _label))
      (Rendering|Material|SetTextureParameterValue _returnvalue_2 "Normal" (Variables|Default|GetNormal))
      (Rendering|Material|SetTextureParameterValue _returnvalue_2 "Masks" (Variables|Default|GetMasks)))
    (:NewEnumerator2
      (Rendering|Material|SetMaterial _gemstone 0 "/Game/FantasticGems/Materials/Instances/MI_Zani_002.MI_Zani_002")
      (goto _label))
    (:NewEnumerator3
      (Rendering|Material|SetMaterial _gemstone 0 "/Game/FantasticGems/Materials/Instances/MI_Zani_003.MI_Zani_003")
      (goto _label))
    (:NewEnumerator4
      (Rendering|Material|SetMaterial _gemstone 0 "/Game/FantasticGems/Materials/Instances/MI_Zani_004.MI_Zani_004")
      (goto _label))
    (:NewEnumerator5
      (Rendering|Material|SetMaterial _gemstone 0 "/Game/FantasticGems/Materials/Instances/MI_Zani_005.MI_Zani_005")
      (goto _label))
    (:NewEnumerator6
      (Rendering|Material|SetMaterial _gemstone 0 "/Game/FantasticGems/Materials/Instances/MI_Zani_006.MI_Zani_006")
      (goto _label))
    (:NewEnumerator7
      (Rendering|Material|SetMaterial _gemstone 0 "/Game/FantasticGems/Materials/Instances/MI_Zani_007.MI_Zani_007")
      (goto _label))
    (:NewEnumerator8
      (Rendering|Material|SetMaterial _gemstone 0 "/Game/FantasticGems/Materials/Instances/MI_Zani_008.MI_Zani_008")
      (goto _label))
    (:NewEnumerator9
      (Rendering|Material|SetMaterial _gemstone 0 "/Game/FantasticGems/Materials/Instances/MI_Zani_009.MI_Zani_009")
      (goto _label))
    (:NewEnumerator10
      (Rendering|Material|SetMaterial _gemstone 0 "/Game/FantasticGems/Materials/Instances/MI_Zani_010.MI_Zani_010")
      (goto _label))))