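; Showcase spawner actor that drops randomly chosen gem actors at random points inside its box volume, with random rotation and scale.
; After a start delay, BeginPlay clears the Stop flag and plays a timeline stretched to StopDelay, then halts both when that time elapses.
; Tick uses a latent Delay as a spawn throttle, with the timeline blending the interval from SpawnIntervals toward a fixed value.
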(event EventBeginPlay
  (bind _timeline_0 (Variables|Default|GetTimeline_0))
  (Utilities|FlowControl|Delay (Variables|Default|GetStart%20Delay))
  (Components|Timeline|SetTimelineLength _timeline_0 (Variables|Default|GetStop%20Delay))
  (Audio|Components|Audio|Play _timeline_0)
  (Variables|Default|SetStop false)
  (Utilities|FlowControl|Delay (Variables|Default|GetStop%20Delay))
  (Variables|Default|SetStop true)
  (Audio|Components|Audio|Stop (Variables|Default|GetTimeline_0)))

(event Collision|EventActorBeginOverlap
  (params (OtherActor :type Actor%20Object%20Reference)))

(event EventTick
  (params (DeltaSeconds :type Float%20%28single-precision%29))
  (bind _returnvalue (Math|Random|RandomFloatinRange 0.6 1.2))
  (bind _gems (Variables|Default|GetGems))
  (bind _volume (Variables|Default|GetVolume))
  (bind _returnvalue_2 (Components|Box|GetScaledBoxExtent _volume))
  (bind (_x _y _z) (Math|Vector|BreakVector _returnvalue_2))
  (if (not (Variables|Default|GetStop))
    (Utilities|FlowControl|Delay (Math|Float|Lerp (Variables|Default|GetSpawnIntervals) 0.3 (stale _newtrack_0)))
    (Game|SpawnActorfromClass (Utilities|Array|Get(acopy) _gems (Math|Random|RandomIntegerinRange 0 (Utilities|Array|LastIndex _gems))) (Math|Transform|MakeTransform (+ (Math|Vector|MakeVector (Math|Random|RandomFloatinRange (* _x -1.0) _x) (Math|Random|RandomFloatinRange (* _y -1.0) _y) (Math|Random|RandomFloatinRange (* _z -1.0) _z)) (Transformation|GetActorLocation)) (Math|Random|RandomRotator true) (Math|Vector|MakeVector _returnvalue _returnvalue _returnvalue)) "Undefined" 0 0)))

(fn ConstructionScript)