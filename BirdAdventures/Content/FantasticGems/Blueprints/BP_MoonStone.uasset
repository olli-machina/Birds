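; Configurable moonstone gem actor whose look is set entirely in the Construction Script, with no runtime logic.
; Freestyle mode creates a dynamic material instance and feeds it exposed variables for textures, sparkles, internal mask rotation, emissive fresnel, subsurface and surface shading.
; Bool and enum options become float switches for the material.
; The ten presets skip material setup and only swap the static mesh to the matching moonstone variant.
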(event EventBeginPlay)

(event Collision|EventActorBeginOverlap
  (params (OtherActor :type Actor%20Object%20Reference)))

(event EventTick
  (params (DeltaSeconds :type Float%20%28single-precision%29)))

(fn ConstructionScript
  (bind _sm_moonstone_001 (Variables|Default|GetSM_Moonstone_001))
  (switch Utilities|FlowControl|Switch|SwitchonENUM_Demon_Eye_001 (Variables|Control|GetFreestyle%20or%20Preset)
    (:NewEnumerator0
      (bind _returnvalue (Rendering|Material|CreateDynamicMaterialInstance _sm_moonstone_001 0 (Rendering|Material|GetMaterial _sm_moonstone_001 0) :!class /Script/Engine.PrimitiveComponent))
      (switch int (Variables|Spark|GetPick%20Sparks%20Texture)
        (:1
          _)
        (:2
          (Rendering|Material|SetTextureParameterValue _returnvalue "Color" "/Game/FantasticGems/Textures/T_Moonstone_002_C.T_Moonstone_002_C"))
        (:3
          (Rendering|Material|SetTextureParameterValue _returnvalue "Color" "/Game/FantasticGems/Textures/T_Moonstone_003_C.T_Moonstone_003_C"))
        (:4
          (Rendering|Material|SetTextureParameterValue _returnvalue "Color" "/Game/FantasticGems/Textures/T_Moonstone_005_C.T_Moonstone_005_C"))
        (:5
          (Rendering|Material|SetTextureParameterValue _returnvalue "Color" "/Game/FantasticGems/Textures/T_Moonstone_004_C.T_Moonstone_004_C"))
        (:6
          (Rendering|Material|SetTextureParameterValue _returnvalue "Color" "/Game/FantasticGems/Textures/T_Moonstone_006_C.T_Moonstone_006_C")))
      (switch int (Variables|Normal|GetPick%20Normal%20Texture)
        (:1
          _)
        (:2
          (Rendering|Material|SetTextureParameterValue _returnvalue "Normal" "/Game/FantasticGems/Textures/T_Maelstrom_001_N.T_Maelstrom_001_N")))
      (Rendering|Material|SetScalarParameterValue _returnvalue "Flipbook Rows" (Variables|Spark|GetSpark%20Row%20Subdivision) :!class /Script/Engine.MaterialInstanceDynamic)
      (Rendering|Material|SetScalarParameterValue _returnvalue "Flipbook Columns" (Variables|Spark|GetSpark%20Column%20Subdivision) :!class /Script/Engine.MaterialInstanceDynamic)
      (Rendering|Material|SetScalarParameterValue _returnvalue "Sparkle Hue" (Variables|Spark|GetSpark%20Hue) :!class /Script/Engine.MaterialInstanceDynamic)
      (Rendering|Material|SetScalarParameterValue _returnvalue "Sparkle Intensity" (Variables|Spark|GetSpark%20Intensity) :!class /Script/Engine.MaterialInstanceDynamic)
      (Rendering|Material|SetScalarParameterValue _returnvalue "Sparkle Desaturation" (Variables|Spark|GetSpark%20Desaturation) :!class /Script/Engine.MaterialInstanceDynamic)
      (Rendering|Material|SetVectorParameterValue _returnvalue "Sparkle Color Multiplier" (Variables|Spark|GetSpark%20Color%20Multiplier) :!class /Script/Engine.MaterialInstanceDynamic)
      (Rendering|Material|SetVectorParameterValue _returnvalue "Color Add" (Variables|Color+Emissive|GetColor%20Add) :!class /Script/Engine.MaterialInstanceDynamic)
      (if (Variables|Spark|GetSpark%20constant%20change)
        (Variables|Spark|SetSpark%20constant%20change_hidden 1.0)
        (else
          (Variables|Spark|SetSpark%20constant%20change_hidden 0.0)))
      (Rendering|Material|SetScalarParameterValue _returnvalue "Use time for sparkles" (Variables|Spark|GetSpark%20constant%20change_hidden) :!class /Script/Engine.MaterialInstanceDynamic)
      (Rendering|Material|SetScalarParameterValue _returnvalue "Sparkle Time Multiplier" (Variables|Spark|GetSpark%20constant%20change%20speed) :!class /Script/Engine.MaterialInstanceDynamic)
      (Rendering|Material|SetScalarParameterValue _returnvalue "Moon Normal Amount" (Variables|Normal|GetNormal%20Intensity) :!class /Script/Engine.MaterialInstanceDynamic)
      (switch Utilities|FlowControl|Switch|SwitchonENUM_Moonstone_001 (Variables|InternalMechanims|GetInternal%20Mask%20Mechanism)
        (:NewEnumerator0
          (Variables|InternalMechanims|SetInternal%20Mask%20mechanism_hidden 0.0))
        (:NewEnumerator1
          (Variables|InternalMechanims|SetInternal%20Mask%20mechanism_hidden 1.0))
        (:NewEnumerator2
          (Variables|InternalMechanims|SetInternal%20Mask%20mechanism_hidden 2.0)))
      (Rendering|Material|SetScalarParameterValue _returnvalue "0= Rotate moon using camera position 1=Rotate moon using time 2=set moon using specific position" (Variables|InternalMechanims|GetInternal%20Mask%20mechanism_hidden) :!class /Script/Engine.MaterialInstanceDynamic)
      (Rendering|Material|SetScalarParameterValue _returnvalue "Time rotation Speed" (Variables|InternalMechanims|GetRotate%20Internal%20map%20on%20loop%20speed) :!class /Script/Engine.MaterialInstanceDynamic)
      (Rendering|Material|SetScalarParameterValue _returnvalue "Specific Position - 0 to 1" (Variables|InternalMechanims|GetInternal%20map%20specific%20position) :!class /Script/Engine.MaterialInstanceDynamic)
      (Rendering|Material|SetScalarParameterValue _returnvalue "Rotate Internal Moon" (Variables|InternalMechanims|GetRotate%20Internal%20map) :!class /Script/Engine.MaterialInstanceDynamic)
      (Rendering|Material|SetScalarParameterValue _returnvalue "Add ulterior rotation based on object direction" (Variables|InternalMechanims|GetAdd%20unterior%20rotation%20based%20on%20objet%20direction) :!class /Script/Engine.MaterialInstanceDynamic)
      (if (Variables|Color+Emissive|GetMultiply%20emissive%20by%20a%20fresnel)
        (Variables|Color+Emissive|SetMultiply%20emissive%20by%20a%20fresnel_hidden 1.0)
        (else
          (Variables|Color+Emissive|SetMultiply%20emissive%20by%20a%20fresnel_hidden 0.0)))
      (Rendering|Material|SetScalarParameterValue _returnvalue "Emissive Fresnel Switch 0 to 1" (Variables|Color+Emissive|GetMultiply%20emissive%20by%20a%20fresnel_hidden) :!class /Script/Engine.MaterialInstanceDynamic)
      (Rendering|Material|SetScalarParameterValue _returnvalue "Emissive Fresnel MIN" (Variables|Color+Emissive|GetEmissive%20Fresnel%20MIN) :!class /Script/Engine.MaterialInstanceDynamic)
      (Rendering|Material|SetScalarParameterValue _returnvalue "Emissive Fresnel MAX" (Variables|Color+Emissive|GetEmissive%20Fresnel%20MAX) :!class /Script/Engine.MaterialInstanceDynamic)
      (Rendering|Material|SetVectorParameterValue _returnvalue "Subsurface Color Add" (Variables|Color+Emissive|GetSubsurface%20Color%20Add) :!class /Script/Engine.MaterialInstanceDynamic)
      (Rendering|Material|SetScalarParameterValue _returnvalue "Subsurface sparkle intensity" (Variables|InternalMechanims|GetIntenal%20Mask%20Subsurface%20intensity) :!class /Script/Engine.MaterialInstanceDynamic)
      (Rendering|Material|SetScalarParameterValue _returnvalue "Moon AO Amount" (Variables|PBR|GetAO%20Amount) :!class /Script/Engine.MaterialInstanceDynamic)
      (Rendering|Material|SetScalarParameterValue _returnvalue "Metallic" (Variables|PBR|GetMetallic%20Amount) :!class /Script/Engine.MaterialInstanceDynamic)
      (Rendering|Material|SetScalarParameterValue _returnvalue "Moon Roughness Amount" (Variables|PBR|GetRoughness%200=simple%201=complex) :!class /Script/Engine.MaterialInstanceDynamic)
      (Rendering|Material|SetScalarParameterValue _returnvalue "Roughness" (Variables|PBR|GetSimple%20Roughness) :!class /Script/Engine.MaterialInstanceDynamic)
      (Rendering|Material|SetScalarParameterValue _returnvalue "Roughness MIN" (Variables|PBR|GetComplex%20Roughness%20MIN) :!class /Script/Engine.MaterialInstanceDynamic)
      (Rendering|Material|SetScalarParameterValue _returnvalue "Roughness MAX" (Variables|PBR|GetComplex%20Roughness%20MAX) :!class /Script/Engine.MaterialInstanceDynamic)
      (Rendering|Material|SetScalarParameterValue _returnvalue "Moon Specular Amount" (Variables|PBR|GetSpecular%200=simple%201=complex) :!class /Script/Engine.MaterialInstanceDynamic)
      (Rendering|Material|SetScalarParameterValue _returnvalue "Specular" (Variables|PBR|GetSimple%20Specular) :!class /Script/Engine.MaterialInstanceDynamic)
      (Rendering|Material|SetScalarParameterValue _returnvalue "Specular MIN" (Variables|PBR|GetComplex%20Specular%20MIN) :!class /Script/Engine.MaterialInstanceDynamic)
      (Rendering|Material|SetScalarParameterValue _returnvalue "Specular MAX" (Variables|PBR|GetComplex%20Specular%20MAX) :!class /Script/Engine.MaterialInstanceDynamic))
    (:NewEnumerator1
      (Components|StaticMesh|SetStaticMesh _sm_moonstone_001 "/Game/FantasticGems/Meshes/SM_Moonstone_001.SM_Moonstone_001"))
    (:NewEnumerator2
      (Components|StaticMesh|SetStaticMesh _sm_moonstone_001 "/Game/FantasticGems/Meshes/SM_Moonstone_002.SM_Moonstone_002"))
    (:NewEnumerator3
      (Components|StaticMesh|SetStaticMesh _sm_moonstone_001 "/Game/FantasticGems/Meshes/SM_Moonstone_003.SM_Moonstone_003"))
    (:NewEnumerator4
      (Components|StaticMesh|SetStaticMesh _sm_moonstone_001 "/Game/FantasticGems/Meshes/SM_Moonstone_004.SM_Moonstone_004"))
    (:NewEnumerator5
      (Components|StaticMesh|SetStaticMesh _sm_moonstone_001 "/Game/FantasticGems/Meshes/SM_Moonstone_005.SM_Moonstone_005"))
    (:NewEnumerator6
      (Components|StaticMesh|SetStaticMesh _sm_moonstone_001 "/Game/FantasticGems/Meshes/SM_Moonstone_006.SM_Moonstone_006"))
    (:NewEnumerator7
      (Components|StaticMesh|SetStaticMesh _sm_moonstone_001 "/Game/FantasticGems/Meshes/SM_Moonstone_007.SM_Moonstone_007"))
    (:NewEnumerator8
      (Components|StaticMesh|SetStaticMesh _sm_moonstone_001 "/Game/FantasticGems/Meshes/SM_Moonstone_008.SM_Moonstone_008"))
    (:NewEnumerator9
      (Components|StaticMesh|SetStaticMesh _sm_moonstone_001 "/Game/FantasticGems/Meshes/SM_Moonstone_009.SM_Moonstone_009"))
    (:NewEnumerator10
      (Components|StaticMesh|SetStaticMesh _sm_moonstone_001 "/Game/FantasticGems/Meshes/SM_Moonstone_010.SM_Moonstone_010"))))