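; Thunderstone gem actor that configures its look in the construction script, either as one of ten preset meshes or freestyle.
; Freestyle builds dynamic material instances on the Gemstone mesh, feeding exposed color, opacity and pulsing emissive values into the gem slot.
; The second slot gets an additive or modulate lightning material with tunable displacement, thickness and emissive colors.
; Presets only swap the static mesh, and the event graph has no runtime logic.
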(event EventBeginPlay)

(event Collision|EventActorBeginOverlap
  (params (OtherActor :type Actor%20Object%20Reference)))

(event EventTick
  (params (DeltaSeconds :type Float%20%28single-precision%29)))

(fn ConstructionScript
  (bind _gemstone (Variables|Default|GetGemstone))
  (bind _gemstone_2 (Variables|Default|GetGemstone))
  (bind _gemstone_3 (Variables|Default|GetGemstone))
  (switch Utilities|FlowControl|Switch|SwitchonENUM_Demon_Eye_001 (Variables|Control|GetFreestyle%20or%20Preset)
    (:NewEnumerator0
      (bind _returnvalue (Rendering|Material|CreateDynamicMaterialInstance _gemstone_2 0 (Rendering|Material|GetMaterial _gemstone_2 0) :!class /Script/Engine.PrimitiveComponent))
      (Rendering|Material|SetScalarParameterValue _returnvalue "Color Hue" (Variables|Color|GetColor%20Hue) :!class /Script/Engine.MaterialInstanceDynamic)
      (Rendering|Material|SetScalarParameterValue _returnvalue "Color Desaturation" (Variables|Color|GetColor%20Desaturation) :!class /Script/Engine.MaterialInstanceDynamic)
      (Rendering|Material|SetVectorParameterValue _returnvalue "Color Multiplier" (Variables|Color|GetColor%20Multiplier) :!class /Script/Engine.MaterialInstanceDynamic)
      (Rendering|Material|SetVectorParameterValue _returnvalue "Emissive color centre" (Variables|Emissive|GetEmissive%20Color%201) :!class /Script/Engine.MaterialInstanceDynamic)
      (Rendering|Material|SetScalarParameterValue _returnvalue "Opacity fresnel 0" (Variables|Opacity|GetOpacity%201) :!class /Script/Engine.MaterialInstanceDynamic)
      (Rendering|Material|SetScalarParameterValue _returnvalue "Opacity fresnel 1" (Variables|Opacity|GetOpacity%202) :!class /Script/Engine.MaterialInstanceDynamic)
      (Rendering|Material|SetScalarParameterValue _returnvalue "Emissive sine speed" (Variables|Emissive|GetEmissive%20Sine%20Speed) :!class /Script/Engine.MaterialInstanceDynamic)
      (Rendering|Material|SetScalarParameterValue _returnvalue "Emissive base" (Variables|Emissive|GetEmisive%20Base%20Intensity) :!class /Script/Engine.MaterialInstanceDynamic)
      (Rendering|Material|SetScalarParameterValue _returnvalue "Emissive sine intensity" (Variables|Emissive|GetEmissive%20Sine%20Intensity) :!class /Script/Engine.MaterialInstanceDynamic)
      (Rendering|Material|SetVectorParameterValue _returnvalue "Emissive sine color" (Variables|Emissive|GetEmissive%20Sine%20Color) :!class /Script/Engine.MaterialInstanceDynamic)
      (Rendering|Material|SetVectorParameterValue _returnvalue "Emissive within" (Variables|Emissive|GetEmissive%20Color%202) :!class /Script/Engine.MaterialInstanceDynamic)
      (switch Utilities|FlowControl|Switch|SwitchonENUM_Thunderstone_001 (Variables|ThunderWithin|GetPick%20Thunder%20Material%20Style)
        (:NewEnumerator0
          (bind _returnvalue_2 (Rendering|Material|CreateDynamicMaterialInstance _gemstone 1 "/Game/FantasticGems/Materials/Master/MAT_Lightning_ADD.MAT_Lightning_ADD" :!class /Script/Engine.PrimitiveComponent))
          (Variables|ThunderWithin|SetThunder%20mat _returnvalue_2))
        (:NewEnumerator1
          (bind _returnvalue_3 (Rendering|Material|CreateDynamicMaterialInstance _gemstone 1 "/Game/FantasticGems/Materials/Master/MAT_Lightning_SUB.MAT_Lightning_SUB" :!class /Script/Engine.PrimitiveComponent))
          (Variables|ThunderWithin|SetThunder%20mat _returnvalue_3)))
      (Rendering|Material|SetScalarParameterValue (Variables|ThunderWithin|GetThunder%20mat) "WPO cLoud INtensity" (Variables|ThunderWithin|GetWPO%20Cloud%20Intensity) :!class /Script/Engine.MaterialInstanceDynamic)
      (Rendering|Material|SetScalarParameterValue (Variables|ThunderWithin|GetThunder%20mat) "WPO Intensity" (Variables|ThunderWithin|GetWPO%20Intensity) :!class /Script/Engine.MaterialInstanceDynamic)
      (Rendering|Material|SetScalarParameterValue (Variables|ThunderWithin|GetThunder%20mat) "Emissive Vertex Color Power" (Variables|ThunderWithin|GetEmissive%20color%20contrast%20intensity) :!class /Script/Engine.MaterialInstanceDynamic)
      (Rendering|Material|SetScalarParameterValue (Variables|ThunderWithin|GetThunder%20mat) "Width Base" (Variables|ThunderWithin|GetThunder%20thickness) :!class /Script/Engine.MaterialInstanceDynamic)
      (Rendering|Material|SetScalarParameterValue (Variables|ThunderWithin|GetThunder%20mat) "Width Tip" (Variables|ThunderWithin|GetThunder%20thickness) :!class /Script/Engine.MaterialInstanceDynamic)
      (Rendering|Material|SetVectorParameterValue (Variables|ThunderWithin|GetThunder%20mat) "Emissive" (Variables|ThunderWithin|GetEmissive%20color%20Within) :!class /Script/Engine.MaterialInstanceDynamic)
      (Rendering|Material|SetVectorParameterValue (Variables|ThunderWithin|GetThunder%20mat) "Emissive Edges" (Variables|ThunderWithin|GetEmissive%20Color%20Edges) :!class /Script/Engine.MaterialInstanceDynamic))
    (:NewEnumerator1
      (Components|StaticMesh|SetStaticMesh _gemstone_3 "/Game/FantasticGems/Meshes/SM_Thunderstone_001.SM_Thunderstone_001"))
    (:NewEnumerator2
      (Components|StaticMesh|SetStaticMesh _gemstone_3 "/Game/FantasticGems/Meshes/SM_Thunderstone_002.SM_Thunderstone_002"))
    (:NewEnumerator3
      (Components|StaticMesh|SetStaticMesh _gemstone_3 "/Game/FantasticGems/Meshes/SM_Thunderstone_003.SM_Thunderstone_003"))
    (:NewEnumerator4
      (Components|StaticMesh|SetStaticMesh _gemstone_3 "/Game/FantasticGems/Meshes/SM_Thunderstone_004.SM_Thunderstone_004"))
    (:NewEnumerator5
      (Components|StaticMesh|SetStaticMesh _gemstone_3 "/Game/FantasticGems/Meshes/SM_Thunderstone_005.SM_Thunderstone_005"))
    (:NewEnumerator6
      (Components|StaticMesh|SetStaticMesh _gemstone_3 "/Game/FantasticGems/Meshes/SM_Thunderstone_006.SM_Thunderstone_006"))
    (:NewEnumerator7
      (Components|StaticMesh|SetStaticMesh _gemstone_3 "/Game/FantasticGems/Meshes/SM_Thunderstone_007.SM_Thunderstone_007"))
    (:NewEnumerator8
      (Components|StaticMesh|SetStaticMesh _gemstone_3 "/Game/FantasticGems/Meshes/SM_Thunderstone_008.SM_Thunderstone_008"))
    (:NewEnumerator9
      (Components|StaticMesh|SetStaticMesh _gemstone_3 "/Game/FantasticGems/Meshes/SM_Thunderstone_009.SM_Thunderstone_009"))
    (:NewEnumerator10
      (Components|StaticMesh|SetStaticMesh _gemstone_3 "/Game/FantasticGems/Meshes/SM_Thunderstone_010.SM_Thunderstone_010"))))