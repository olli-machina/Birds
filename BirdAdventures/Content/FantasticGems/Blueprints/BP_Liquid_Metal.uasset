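; Configurable liquid metal gemstone actor, set up entirely in the construction script with no active runtime logic.
; FreestyleOrPreset either swaps the Gemstone component to one of ten preset meshes or, in Freestyle, creates a dynamic material instance from its current material.
; Freestyle feeds exposed variables into that material: texture picks, colors, surface properties, speeds, RGB channel selectors for FX, and World Position Offset intensity.
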(event EventBeginPlay)

(event Collision|EventActorBeginOverlap
  (params (OtherActor :type Actor%20Object%20Reference)))

(event EventTick
  (params (DeltaSeconds :type Float%20%28single-precision%29)))

(fn ConstructionScript
  (bind _gemstone (Variables|Default|GetGemstone))
  (bind _gemstone_2 (Variables|Default|GetGemstone))
  (switch Utilities|FlowControl|Switch|SwitchonENUM_Demon_Eye_001 (Variables|Control|GetFreestyle%20or%20Preset)
    (:NewEnumerator0
      (bind _returnvalue (Rendering|Material|CreateDynamicMaterialInstance _gemstone 0 (Rendering|Material|GetMaterial _gemstone 0) :!class /Script/Engine.PrimitiveComponent))
      (Variables|Control|SetNewVar_0 _returnvalue)
      (switch int (Variables|Normal|GetPick%20Normal%20Texture)
        (:1
          (Rendering|Material|SetTextureParameterValue _returnvalue "Normal" "/Game/FantasticGems/Textures/T_Liquid_Metal_001N.T_Liquid_Metal_001N"))
        (:2
          (Rendering|Material|SetTextureParameterValue _returnvalue "Normal" "/Game/FantasticGems/Textures/T_Liquid_Metal_002_N.T_Liquid_Metal_002_N"))
        (:3
          (Rendering|Material|SetTextureParameterValue _returnvalue "Normal" "/Game/FantasticGems/Textures/T_Liquid_Metal_003_N.T_Liquid_Metal_003_N")))
      (Rendering|Material|SetScalarParameterValue _returnvalue "Use Texture - Normal" (Variables|Normal|GetUse%20Normal%20Texture) :!class /Script/Engine.MaterialInstanceDynamic)
      (switch int (Variables|Color|GetPick%20Color%20Texture)
        (:1
          (Rendering|Material|SetTextureParameterValue (Variables|Control|GetNewVar_0) "Color" "/Game/FantasticGems/Textures/T_Liquid_Metal_001_C.T_Liquid_Metal_001_C"))
        (:2
          (Rendering|Material|SetTextureParameterValue (Variables|Control|GetNewVar_0) "Color" "/Game/FantasticGems/Textures/T_Liquid_Metal_002_C.T_Liquid_Metal_002_C"))
        (:3
          (Rendering|Material|SetTextureParameterValue (Variables|Control|GetNewVar_0) "Color" "/Game/FantasticGems/Textures/T_Liquid_Metal_003_C.T_Liquid_Metal_003_C")))
      (Rendering|Material|SetScalarParameterValue (Variables|Control|GetNewVar_0) "Use Texture - Color" (Variables|Color|GetUse%20Color%20Texture) :!class /Script/Engine.MaterialInstanceDynamic)
      (Rendering|Material|SetVectorParameterValue _returnvalue "Color" (Variables|Color|GetColor%201) :!class /Script/Engine.MaterialInstanceDynamic)
      (Rendering|Material|SetVectorParameterValue (Variables|Control|GetNewVar_0) "Color 2" (Variables|Color|GetColor%202) :!class /Script/Engine.MaterialInstanceDynamic)
      (Rendering|Material|SetVectorParameterValue (Variables|Control|GetNewVar_0) "Color Multiplier 1" (Variables|Color|GetColor%20Multiplier%201) :!class /Script/Engine.MaterialInstanceDynamic)
      (Rendering|Material|SetVectorParameterValue (Variables|Control|GetNewVar_0) "Color Multiplier 2" (Variables|Color|GetColor%20Multiplier%202) :!class /Script/Engine.MaterialInstanceDynamic)
      (Rendering|Material|SetScalarParameterValue (Variables|Control|GetNewVar_0) "Color multiplier contrast" (Variables|Color|GetColor%20Multiplier%20Contrast) :!class /Script/Engine.MaterialInstanceDynamic)
      (Rendering|Material|SetScalarParameterValue (Variables|Control|GetNewVar_0) "Use Texture - Roughness" (Variables|Masks|GetUse%20Roughness%20Texture) :!class /Script/Engine.MaterialInstanceDynamic)
      (Rendering|Material|SetScalarParameterValue (Variables|Control|GetNewVar_0) "Roughness 1" (Variables|Masks|GetRoughness%201) :!class /Script/Engine.MaterialInstanceDynamic)
      (Rendering|Material|SetScalarParameterValue (Variables|Control|GetNewVar_0) "Roughness 2" (Variables|Masks|GetRoughness%202) :!class /Script/Engine.MaterialInstanceDynamic)
      (Rendering|Material|SetScalarParameterValue (Variables|Control|GetNewVar_0) "Use Texture - Metal" (Variables|Masks|GetUse%20Metal%20Texture) :!class /Script/Engine.MaterialInstanceDynamic)
      (Rendering|Material|SetScalarParameterValue (Variables|Control|GetNewVar_0) "Use Texture - AO" (Variables|Masks|GetUse%20AO%20Texture) :!class /Script/Engine.MaterialInstanceDynamic)
      (Rendering|Material|SetScalarParameterValue (Variables|Control|GetNewVar_0) "AO" (Variables|Masks|GetAO) :!class /Script/Engine.MaterialInstanceDynamic)
      (Rendering|Material|SetScalarParameterValue (Variables|Control|GetNewVar_0) "Metal" (Variables|Masks|GetMetal) :!class /Script/Engine.MaterialInstanceDynamic)
      (switch int (Variables|Masks|GetPick%20Masks%20Texture)
        (:1
          (Rendering|Material|SetTextureParameterValue (Variables|Control|GetNewVar_0) "Masks" "/Game/FantasticGems/Textures/T_Liquid_Metal_001_S.T_Liquid_Metal_001_S"))
        (:2
          (Rendering|Material|SetTextureParameterValue (Variables|Control|GetNewVar_0) "Masks" "/Game/FantasticGems/Textures/T_Liquid_Metal_002_S.T_Liquid_Metal_002_S"))
        (:3
          (Rendering|Material|SetTextureParameterValue (Variables|Control|GetNewVar_0) "Masks" "/Game/FantasticGems/Textures/T_Liquid_Metal_003_S.T_Liquid_Metal_003_S")))
      (switch int (Variables|WPO|GetPick%20FX%20Texture)
        (:1
          (Rendering|Material|SetTextureParameterValue (Variables|Control|GetNewVar_0) "FX" "/Game/FantasticGems/Textures/T_Liquid_Metal_M_001.T_Liquid_Metal_M_001"))
        (:2
          (Rendering|Material|SetTextureParameterValue (Variables|Control|GetNewVar_0) "FX" "/Game/FantasticGems/Textures/T_Liquid_Metal_M_002.T_Liquid_Metal_M_002")))
      (Rendering|Material|SetScalarParameterValue (Variables|Control|GetNewVar_0) "Speed 1" (Variables|WPO|GetSpeed%201) :!class /Script/Engine.MaterialInstanceDynamic)
      (Rendering|Material|SetScalarParameterValue (Variables|Control|GetNewVar_0) "Speed 2" (Variables|WPO|GetSpeed%202) :!class /Script/Engine.MaterialInstanceDynamic)
      (Rendering|Material|SetScalarParameterValue (Variables|Control|GetNewVar_0) "Speed 3" (Variables|WPO|GetSpeed%203) :!class /Script/Engine.MaterialInstanceDynamic)
      (Rendering|Material|SetScalarParameterValue (Variables|Control|GetNewVar_0) "Speed 4" (Variables|WPO|GetSpeed%204) :!class /Script/Engine.MaterialInstanceDynamic)
      (Rendering|Material|SetScalarParameterValue (Variables|Control|GetNewVar_0) "FX 1 0=R 1=G 2=B" (Math|Conversions|ToFloat(Integer) (Variables|WPO|GetFX%20Selector%201)) :!class /Script/Engine.MaterialInstanceDynamic)
      (Rendering|Material|SetScalarParameterValue (Variables|Control|GetNewVar_0) "FX 2 0=R 1=G 2=B" (Math|Conversions|ToFloat(Integer) (Variables|WPO|GetFX%20Selector%202)) :!class /Script/Engine.MaterialInstanceDynamic)
      (Rendering|Material|SetScalarParameterValue (Variables|Control|GetNewVar_0) "WPO Intensity" (Variables|WPO|GetWPO%20Intensity) :!class /Script/Engine.MaterialInstanceDynamic))
    (:NewEnumerator1
      (Components|StaticMesh|SetStaticMesh _gemstone_2 "/Game/FantasticGems/Meshes/SM_Liquid_Metal_001.SM_Liquid_Metal_001"))
    (:NewEnumerator2
      (Components|StaticMesh|SetStaticMesh _gemstone_2 "/Game/FantasticGems/Meshes/SM_Liquid_Metal_002.SM_Liquid_Metal_002"))
    (:NewEnumerator3
      (Components|StaticMesh|SetStaticMesh _gemstone_2 "/Game/FantasticGems/Meshes/SM_Liquid_Metal_003.SM_Liquid_Metal_003"))
    (:NewEnumerator4
      (Components|StaticMesh|SetStaticMesh _gemstone_2 "/Game/FantasticGems/Meshes/SM_Liquid_Metal_004.SM_Liquid_Metal_004"))
    (:NewEnumerator5
      (Components|StaticMesh|SetStaticMesh _gemstone_2 "/Game/FantasticGems/Meshes/SM_Liquid_Metal_005.SM_Liquid_Metal_005"))
    (:NewEnumerator6
      (Components|StaticMesh|SetStaticMesh _gemstone_2 "/Game/FantasticGems/Meshes/SM_Liquid_Metal_006.SM_Liquid_Metal_006"))
    (:NewEnumerator7
      (Components|StaticMesh|SetStaticMesh _gemstone_2 "/Game/FantasticGems/Meshes/SM_Liquid_Metal_007.SM_Liquid_Metal_007"))
    (:NewEnumerator8
      (Components|StaticMesh|SetStaticMesh _gemstone_2 "/Game/FantasticGems/Meshes/SM_Liquid_Metal_008.SM_Liquid_Metal_008"))
    (:NewEnumerator9
      (Components|StaticMesh|SetStaticMesh _gemstone_2 "/Game/FantasticGems/Meshes/SM_Liquid_Metal_009.SM_Liquid_Metal_009"))
    (:NewEnumerator10
      (Components|StaticMesh|SetStaticMesh _gemstone_2 "/Game/FantasticGems/Meshes/SM_Liquid_Metal_010.SM_Liquid_Metal_010"))))