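; Configurable Sloe gemstone actor from FantasticGems that sets up its look entirely in the Construction Script, with no runtime logic.
; Freestyle mode creates a dynamic material instance and pushes exposed variables for WPO spikes and pulsing, cloud motion, colors, subsurface, normals, specular and roughness.
; ChangeFX picks one of three FX and detail normal texture pairs.
; Presets instead swap the Gemstone mesh among ten variants and create a material instance without overrides.
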(event EventBeginPlay)

(event Collision|EventActorBeginOverlap
  (params (OtherActor :type Actor%20Object%20Reference)))

(event EventTick
  (params (DeltaSeconds :type Float%20%28single-precision%29)))

(fn ConstructionScript
  (bind _gemstone (Variables|Default|GetGemstone))
  (bind _gemstone_2 (Variables|Default|GetGemstone))
  (bind _gemstone_3 (Variables|Default|GetGemstone))
  (switch Utilities|FlowControl|Switch|SwitchonENUM_Demon_Eye_001 (Variables|Control|GetFreestyle%20or%20Preset)
    (:NewEnumerator0
      (bind _returnvalue (Rendering|Material|CreateDynamicMaterialInstance _gemstone_2 0 (Rendering|Material|GetMaterial _gemstone_2 0) :!class /Script/Engine.PrimitiveComponent))
      (switch int (Variables|Control|GetChange%20FX)
        (:1
          (Rendering|Material|SetTextureParameterValue _returnvalue "FX" "/Game/FantasticGems/Textures/T_Sloe_001_M.T_Sloe_001_M")
          (Rendering|Material|SetTextureParameterValue _returnvalue "Detail Normal" "/Game/FantasticGems/Textures/T_Sloe_001_N.T_Sloe_001_N"))
        (:2
          (Rendering|Material|SetTextureParameterValue _returnvalue "FX" "/Game/FantasticGems/Textures/T_Sloe_002_M.T_Sloe_002_M")
          (Rendering|Material|SetTextureParameterValue _returnvalue "Detail Normal" "/Game/FantasticGems/Textures/T_Sloe_002_N.T_Sloe_002_N"))
        (:3
          (Rendering|Material|SetTextureParameterValue _returnvalue "FX" "/Game/FantasticGems/Textures/T_Sloe_003_M.T_Sloe_003_M")
          (Rendering|Material|SetTextureParameterValue _returnvalue "Detail Normal" "/Game/FantasticGems/Textures/T_Sloe_004_N.T_Sloe_004_N")))
      (Rendering|Material|SetScalarParameterValue _returnvalue "Use spikes" (Variables|WPO|GetUse%20world%20Position%20Offset%20%28WPO%29) :!class /Script/Engine.MaterialInstanceDynamic)
      (Rendering|Material|SetScalarParameterValue _returnvalue "Use Vertex Color" (Variables|WPO|GetUse%20Vertex%20color%20with%20WPO%20%28spikes%29) :!class /Script/Engine.MaterialInstanceDynamic)
      (Rendering|Material|SetScalarParameterValue _returnvalue "Spikes intensity" (Variables|WPO|GetWPO%20Intensity) :!class /Script/Engine.MaterialInstanceDynamic)
      (Rendering|Material|SetScalarParameterValue _returnvalue "Use sine" (Variables|WPO|GetAdd%20a%20sine%20to%20WPO%20%28pulsing%29) :!class /Script/Engine.MaterialInstanceDynamic)
      (Rendering|Material|SetScalarParameterValue _returnvalue "Time Spikes intensity add" (Variables|WPO|GetWPO%20Pulse%20Intensity) :!class /Script/Engine.MaterialInstanceDynamic)
      (Rendering|Material|SetScalarParameterValue _returnvalue "Time speed" (Variables|WPO|GetWPO%20Pulse%20Speed) :!class /Script/Engine.MaterialInstanceDynamic)
      (Rendering|Material|SetScalarParameterValue _returnvalue "Add cloud to WPO" (Variables|WPO|GetAdd%20cloud%20to%20WPO) :!class /Script/Engine.MaterialInstanceDynamic)
      (Rendering|Material|SetScalarParameterValue _returnvalue "FX Cloud UVs" (Variables|WPO|GetCloud%20UV%20Scale) :!class /Script/Engine.MaterialInstanceDynamic)
      (Rendering|Material|SetScalarParameterValue _returnvalue "Movement Speed 1" (Variables|WPO|GetCloud%20Speed%201) :!class /Script/Engine.MaterialInstanceDynamic)
      (Rendering|Material|SetScalarParameterValue _returnvalue "Movement Speed 2" (Variables|WPO|GetCloud%20Speed%202) :!class /Script/Engine.MaterialInstanceDynamic)
      (Rendering|Material|SetVectorParameterValue _returnvalue "Color Rim" (Variables|Color|GetRim%20Color) :!class /Script/Engine.MaterialInstanceDynamic)
      (Rendering|Material|SetVectorParameterValue _returnvalue "Color Add" (Variables|Color|GetColor%20Add) :!class /Script/Engine.MaterialInstanceDynamic)
      (Rendering|Material|SetVectorParameterValue _returnvalue "Subsurface Color Rim" (Variables|Color|GetRim%20Subsurface%20Color) :!class /Script/Engine.MaterialInstanceDynamic)
      (Rendering|Material|SetVectorParameterValue _returnvalue "Subsurface Color Add" (Variables|Color|GetSubsurface%20Color%20Add) :!class /Script/Engine.MaterialInstanceDynamic)
      (Rendering|Material|SetScalarParameterValue _returnvalue "Detail Normal Map Intensity" (Variables|Normal|GetDetail%20Normal%20Intensity) :!class /Script/Engine.MaterialInstanceDynamic)
      (Rendering|Material|SetScalarParameterValue _returnvalue "Normal Map Intensity" (Variables|Normal|GetNormal%20Intensity) :!class /Script/Engine.MaterialInstanceDynamic)
      (Rendering|Material|SetScalarParameterValue _returnvalue "Detail Normal Speed 1" (Variables|Normal|GetDetail%20Normal%20Speed%201) :!class /Script/Engine.MaterialInstanceDynamic)
      (Rendering|Material|SetScalarParameterValue _returnvalue "Detail Normal Speed 2" (Variables|Normal|GetDetail%20Normal%20Speed%202) :!class /Script/Engine.MaterialInstanceDynamic)
      (Rendering|Material|SetScalarParameterValue _returnvalue "Detail Normal UV Scale" (Variables|Normal|GetDetail%20Normal%20UV%20Scale) :!class /Script/Engine.MaterialInstanceDynamic)
      (Rendering|Material|SetScalarParameterValue _returnvalue "Specular MIN" (Variables|BPR|GetSpecular%20MIN) :!class /Script/Engine.MaterialInstanceDynamic)
      (Rendering|Material|SetScalarParameterValue _returnvalue "Specular MAX" (Variables|BPR|GetSpecular%20MAX) :!class /Script/Engine.MaterialInstanceDynamic)
      (Rendering|Material|SetScalarParameterValue _returnvalue "Roughness MIN" (Variables|BPR|GetRoughness%20MIN) :!class /Script/Engine.MaterialInstanceDynamic)
      (Rendering|Material|SetScalarParameterValue _returnvalue "Roughness MAX" (Variables|BPR|GetRoughness%20MAX) :!class /Script/Engine.MaterialInstanceDynamic)
      (Rendering|Material|SetScalarParameterValue _returnvalue "Roughness Rim" (Variables|BPR|GetRoughness%20Rim) :!class /Script/Engine.MaterialInstanceDynamic))
    (:NewEnumerator1
      (Components|StaticMesh|SetStaticMesh _gemstone_3 "/Game/FantasticGems/Meshes/SM_Sloe_001.SM_Sloe_001")
      (Rendering|Material|CreateDynamicMaterialInstance _gemstone 0 (Rendering|Material|GetMaterial _gemstone 0) :!class /Script/Engine.PrimitiveComponent :!label _label))
    (:NewEnumerator2
      (Components|StaticMesh|SetStaticMesh _gemstone_3 "/Game/FantasticGems/Meshes/SM_Sloe_002.SM_Sloe_002")
      (goto _label))
    (:NewEnumerator3
      (Components|StaticMesh|SetStaticMesh _gemstone_3 "/Game/FantasticGems/Meshes/SM_Sloe_003.SM_Sloe_003")
      (goto _label))
    (:NewEnumerator4
      (Components|StaticMesh|SetStaticMesh _gemstone_3 "/Game/FantasticGems/Meshes/SM_Sloe_004.SM_Sloe_004")
      (goto _label))
    (:NewEnumerator5
      (Components|StaticMesh|SetStaticMesh _gemstone_3 "/Game/FantasticGems/Meshes/SM_Sloe_005.SM_Sloe_005")
      (goto _label))
    (:NewEnumerator6
      (Components|StaticMesh|SetStaticMesh _gemstone_3 "/Game/FantasticGems/Meshes/SM_Sloe_006.SM_Sloe_006")
      (goto _label))
    (:NewEnumerator7
      (Components|StaticMesh|SetStaticMesh _gemstone_3 "/Game/FantasticGems/Meshes/SM_Sloe_007.SM_Sloe_007")
      (goto _label))
    (:NewEnumerator8
      (Components|StaticMesh|SetStaticMesh _gemstone_3 "/Game/FantasticGems/Meshes/SM_Sloe_008.SM_Sloe_008")
      (goto _label))
    (:NewEnumerator9
      (Components|StaticMesh|SetStaticMesh _gemstone_3 "/Game/FantasticGems/Meshes/SM_Sloe_009.SM_Sloe_009")
      (goto _label))
    (:NewEnumerator10
      (Components|StaticMesh|SetStaticMesh _gemstone_3 "/Game/FantasticGems/Meshes/SM_Sloe_010.SM_Sloe_010")
      (goto _label))))