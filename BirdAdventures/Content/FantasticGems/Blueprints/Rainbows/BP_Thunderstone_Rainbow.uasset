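; Thunderstone gemstone Blueprint that animates a rainbow hue shift on its materials during play.
; The construction script picks one of the numbered Thunderstone meshes from Seed, leaving the component's mesh unchanged for values without a case.
; On BeginPlay, a timeline with RainbowSpeed as play rate drives hue parameters on dynamic materials in two slots.
; The second slot's dynamic instance is created inside every timeline update rather than once.
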(event EventBeginPlay
  (bind _gemstone (Variables|Default|GetGemstone))
  (bind _gemstone_2 (Variables|Default|GetGemstone))
  (Components|Timeline|SetPlayRate (Variables|Default|GetRainbow_Timeline) (Variables|Default|GetRainbow%20Speed))
  (bind _returnvalue (Rendering|Material|CreateDynamicMaterialInstance _gemstone 0 (Rendering|Material|GetMaterial _gemstone 0) :!class /Script/Engine.PrimitiveComponent))
  (bind _hue (Timeline|Rainbow_Timeline Play)
    (:Update
      (Rendering|Material|SetScalarParameterValue _returnvalue "Color Hue" _hue :!class /Script/Engine.MaterialInstanceDynamic)
      (bind _returnvalue_2 (Rendering|Material|CreateDynamicMaterialInstance _gemstone_2 1 (Rendering|Material|GetMaterial _gemstone_2 1) :!class /Script/Engine.PrimitiveComponent))
      (Rendering|Material|SetScalarParameterValue _returnvalue_2 "hue" _hue :!class /Script/Engine.MaterialInstanceDynamic))))

(fn ConstructionScript
  (bind _gemstone (Variables|Default|GetGemstone))
  (switch int (Variables|Default|GetSeed)
    (:2
      (Components|StaticMesh|SetStaticMesh _gemstone "/Game/FantasticGems/Meshes/SM_Thunderstone_002.SM_Thunderstone_002"))
    (:3
      (Components|StaticMesh|SetStaticMesh _gemstone "/Game/FantasticGems/Meshes/SM_Thunderstone_003.SM_Thunderstone_003"))
    (:4
      (Components|StaticMesh|SetStaticMesh _gemstone "/Game/FantasticGems/Meshes/SM_Thunderstone_004.SM_Thunderstone_004"))
    (:5
      (Components|StaticMesh|SetStaticMesh _gemstone "/Game/FantasticGems/Meshes/SM_Thunderstone_005.SM_Thunderstone_005"))
    (:6
      (Components|StaticMesh|SetStaticMesh _gemstone "/Game/FantasticGems/Meshes/SM_Thunderstone_006.SM_Thunderstone_006"))
    (:7
      (Components|StaticMesh|SetStaticMesh _gemstone "/Game/FantasticGems/Meshes/SM_Thunderstone_007.SM_Thunderstone_007"))
    (:8
      (Components|StaticMesh|SetStaticMesh _gemstone "/Game/FantasticGems/Meshes/SM_Thunderstone_008.SM_Thunderstone_008"))
    (:9
      (Components|StaticMesh|SetStaticMesh _gemstone "/Game/FantasticGems/Meshes/SM_Thunderstone_009.SM_Thunderstone_009"))
    (:10
      (Components|StaticMesh|SetStaticMesh _gemstone "/Game/FantasticGems/Meshes/SM_Thunderstone_010.SM_Thunderstone_010"))))