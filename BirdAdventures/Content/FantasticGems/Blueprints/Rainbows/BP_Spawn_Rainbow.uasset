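; Gemstone spawn prop whose colour shifts by animating material hue, in one of several mesh variants.
; The construction script picks the SM_Spawn mesh from Seed, leaving the default mesh for unlisted values.
; On BeginPlay, a timeline at RainbowSpeed drives the Hue parameter on dynamic materials in three slots.
; Slot 2's instance is created once, while the create call for slots 1 and 0 runs every update.
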(event EventBeginPlay
  (bind _gemstone (Variables|Default|GetGemstone))
  (bind _gemstone_2 (Variables|Default|GetGemstone))
  (bind _gemstone_3 (Variables|Default|GetGemstone))
  (Components|Timeline|SetPlayRate (Variables|Default|GetRainbow_Timeline) (Variables|Default|GetRainbow%20Speed))
  (bind _returnvalue (Rendering|Material|CreateDynamicMaterialInstance _gemstone 2 (Rendering|Material|GetMaterial _gemstone 2) :!class /Script/Engine.PrimitiveComponent))
  (bind _hue (Timeline|Rainbow_Timeline Play)
    (:Update
      (Rendering|Material|SetScalarParameterValue _returnvalue "Hue" _hue :!class /Script/Engine.MaterialInstanceDynamic)
      (bind _returnvalue_2 (Rendering|Material|CreateDynamicMaterialInstance _gemstone_2 1 (Rendering|Material|GetMaterial _gemstone_2 1) :!class /Script/Engine.PrimitiveComponent))
      (Rendering|Material|SetScalarParameterValue _returnvalue_2 "Hue" _hue :!class /Script/Engine.MaterialInstanceDynamic)
      (bind _returnvalue_3 (Rendering|Material|CreateDynamicMaterialInstance _gemstone_3 0 (Rendering|Material|GetMaterial _gemstone_3 0) :!class /Script/Engine.PrimitiveComponent))
      (Rendering|Material|SetScalarParameterValue _returnvalue_3 "Hue" _hue :!class /Script/Engine.MaterialInstanceDynamic))))

(fn ConstructionScript
  (bind _gemstone (Variables|Default|GetGemstone))
  (switch int (Variables|Default|GetSeed)
    (:2
      (Components|StaticMesh|SetStaticMesh _gemstone "/Game/FantasticGems/Meshes/SM_Spawn_002.SM_Spawn_002"))
    (:3
      (Components|StaticMesh|SetStaticMesh _gemstone "/Game/FantasticGems/Meshes/SM_Spawn_003.SM_Spawn_003"))
    (:4
      (Components|StaticMesh|SetStaticMesh _gemstone "/Game/FantasticGems/Meshes/SM_Spawn_004.SM_Spawn_004"))
    (:5
      (Components|StaticMesh|SetStaticMesh _gemstone "/Game/FantasticGems/Meshes/SM_Spawn_005.SM_Spawn_005"))
    (:6
      (Components|StaticMesh|SetStaticMesh _gemstone "/Game/FantasticGems/Meshes/SM_Spawn_006.SM_Spawn_006"))
    (:7
      (Components|StaticMesh|SetStaticMesh _gemstone "/Game/FantasticGems/Meshes/SM_Spawn_007.SM_Spawn_007"))
    (:8
      (Components|StaticMesh|SetStaticMesh _gemstone "/Game/FantasticGems/Meshes/SM_Spawn_008.SM_Spawn_008"))
    (:9
      (Components|StaticMesh|SetStaticMesh _gemstone "/Game/FantasticGems/Meshes/SM_Spawn_009.SM_Spawn_009"))
    (:10
      (Components|StaticMesh|SetStaticMesh _gemstone "/Game/FantasticGems/Meshes/SM_Spawn_010.SM_Spawn_010"))))