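; BP_Demon_Rainbow is a demon-eye gemstone actor that animates its hue for a rainbow effect.
; The Construction Script picks one of several demon-eye static meshes for the Gemstone component from the Seed value.
; On BeginPlay it creates a dynamic material instance from the gem's material, and a timeline with play rate set by RainbowSpeed drives that instance's Hue parameter.
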(event EventBeginPlay
  (bind _gemstone (Variables|Default|GetGemstone))
  (Components|Timeline|SetPlayRate (Variables|Default|GetRainbow_Timeline) (Variables|Default|GetRainbow%20Speed))
  (bind _returnvalue (Rendering|Material|CreateDynamicMaterialInstance _gemstone 0 (Rendering|Material|GetMaterial _gemstone 0) :!class /Script/Engine.PrimitiveComponent))
  (bind _hue (Timeline|Rainbow_Timeline Play)
    (:Update
      (Rendering|Material|SetScalarParameterValue _returnvalue "Hue" _hue :!class /Script/Engine.MaterialInstanceDynamic))))

(fn ConstructionScript
  (bind _gemstone (Variables|Default|GetGemstone))
  (switch int (Variables|Default|GetSeed)
    (:2
      (Components|StaticMesh|SetStaticMesh _gemstone "/Game/FantasticGems/Meshes/SM_Demon_Eye_001.SM_Demon_Eye_001"))
    (:3
      (Components|StaticMesh|SetStaticMesh _gemstone "/Game/FantasticGems/Meshes/SM_Demon_Eye_002.SM_Demon_Eye_002"))
    (:4
      (Components|StaticMesh|SetStaticMesh _gemstone "/Game/FantasticGems/Meshes/SM_Demon_Eye_003.SM_Demon_Eye_003"))
    (:5
      (Components|StaticMesh|SetStaticMesh _gemstone "/Game/FantasticGems/Meshes/SM_Demon_Eye_004.SM_Demon_Eye_004"))
    (:6
      (Components|StaticMesh|SetStaticMesh _gemstone "/Game/FantasticGems/Meshes/SM_Demon_Eye_006.SM_Demon_Eye_006"))
    (:7
      (Components|StaticMesh|SetStaticMesh _gemstone "/Game/FantasticGems/Meshes/SM_Demon_Eye_007.SM_Demon_Eye_007"))
    (:8
      (Components|StaticMesh|SetStaticMesh _gemstone "/Game/FantasticGems/Meshes/SM_Demon_Eye_008.SM_Demon_Eye_008"))
    (:9
      (Components|StaticMesh|SetStaticMesh _gemstone "/Game/FantasticGems/Meshes/SM_Demon_Eye_009.SM_Demon_Eye_009"))
    (:10
      (Components|StaticMesh|SetStaticMesh _gemstone "/Game/FantasticGems/Meshes/SM_Demon_Eye_010.SM_Demon_Eye_010"))))