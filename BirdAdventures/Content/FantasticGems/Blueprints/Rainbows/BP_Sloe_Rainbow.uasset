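; Sloe gemstone actor that animates a rainbow color effect.
; The construction script picks one of the sloe mesh variants from Seed, leaving the component's mesh unchanged for values outside the handled cases.
; On BeginPlay it creates a dynamic material from the gemstone's first material slot, and a timeline with play rate set by RainbowSpeed drives its Hue parameter.
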(event EventBeginPlay
  (bind _gemstone (Variables|Default|GetGemstone))
  (Components|Timeline|SetPlayRate (Variables|Default|GetRainbow_Timeline) (Variables|Default|GetRainbow%20Speed))
  (bind _returnvalue (Rendering|Material|CreateDynamicMaterialInstance _gemstone 0 (Rendering|Material|GetMaterial _gemstone 0) :!class /Script/Engine.PrimitiveComponent))
  (bind _hue (Timeline|Rainbow_Timeline Play)
    (:Update
      (Rendering|Material|SetScalarParameterValue _returnvalue "Hue" _hue :!class /Script/Engine.MaterialInstanceDynamic))))

(fn ConstructionScript
  (bind _gemstone (Variables|Default|GetGemstone))
  (switch int (Variables|Default|GetSeed)
    (:2
      (Components|StaticMesh|SetStaticMesh _gemstone "/Game/FantasticGems/Meshes/SM_Sloe_002.SM_Sloe_002"))
    (:3
      (Components|StaticMesh|SetStaticMesh _gemstone "/Game/FantasticGems/Meshes/SM_Sloe_003.SM_Sloe_003"))
    (:4
      (Components|StaticMesh|SetStaticMesh _gemstone "/Game/FantasticGems/Meshes/SM_Sloe_004.SM_Sloe_004"))
    (:5
      (Components|StaticMesh|SetStaticMesh _gemstone "/Game/FantasticGems/Meshes/SM_Sloe_005.SM_Sloe_005"))
    (:6
      (Components|StaticMesh|SetStaticMesh _gemstone "/Game/FantasticGems/Meshes/SM_Sloe_006.SM_Sloe_006"))
    (:7
      (Components|StaticMesh|SetStaticMesh _gemstone "/Game/FantasticGems/Meshes/SM_Sloe_007.SM_Sloe_007"))
    (:8
      (Components|StaticMesh|SetStaticMesh _gemstone "/Game/FantasticGems/Meshes/SM_Sloe_008.SM_Sloe_008"))
    (:9
      (Components|StaticMesh|SetStaticMesh _gemstone "/Game/FantasticGems/Meshes/SM_Sloe_009.SM_Sloe_009"))
    (:10
      (Components|StaticMesh|SetStaticMesh _gemstone "/Game/FantasticGems/Meshes/SM_Sloe_010.SM_Sloe_010"))))