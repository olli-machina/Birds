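; BP_Jesper_Rainbow is a Jesper gemstone actor whose color continuously shifts through hues for a rainbow effect.
; The construction script picks one of several Jesper static meshes from the Seed value.
; On BeginPlay it creates a dynamic material instance on the Gemstone mesh and plays a timeline at RainbowSpeed.
; The timeline's Hue track drives both the Color Hue and Subsurface Hue parameters.
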(event EventBeginPlay
  (bind _gemstone (Variables|Default|GetGemstone))
  (Components|Timeline|SetPlayRate (Variables|Default|GetRainbow_Timeline) (Variables|Default|GetRainbow%20Speed))
  (bind _returnvalue (Rendering|Material|CreateDynamicMaterialInstance _gemstone 0 (Rendering|Material|GetMaterial _gemstone 0) :!class /Script/Engine.PrimitiveComponent))
  (bind _hue (Timeline|Rainbow_Timeline Play)
    (:Update
      (Rendering|Material|SetScalarParameterValue _returnvalue "Subsurface Hue" _hue :!class /Script/Engine.MaterialInstanceDynamic)
      (Rendering|Material|SetScalarParameterValue _returnvalue "Color Hue" _hue :!class /Script/Engine.MaterialInstanceDynamic))))

(fn ConstructionScript
  (bind _gemstone (Variables|Default|GetGemstone))
  (switch int (Variables|Default|GetSeed)
    (:2
      (Components|StaticMesh|SetStaticMesh _gemstone "/Game/FantasticGems/Meshes/SM_Jesper_002.SM_Jesper_002"))
    (:3
      (Components|StaticMesh|SetStaticMesh _gemstone "/Game/FantasticGems/Meshes/SM_Jesper_003.SM_Jesper_003"))
    (:4
      (Components|StaticMesh|SetStaticMesh _gemstone "/Game/FantasticGems/Meshes/SM_Jesper_004.SM_Jesper_004"))
    (:5
      (Components|StaticMesh|SetStaticMesh _gemstone "/Game/FantasticGems/Meshes/SM_Jesper_005.SM_Jesper_005"))
    (:6
      (Components|StaticMesh|SetStaticMesh _gemstone "/Game/FantasticGems/Meshes/SM_Jesper_006.SM_Jesper_006"))
    (:7
      (Components|StaticMesh|SetStaticMesh _gemstone "/Game/FantasticGems/Meshes/SM_Jesper_007.SM_Jesper_007"))
    (:8
      (Components|StaticMesh|SetStaticMesh _gemstone "/Game/FantasticGems/Meshes/SM_Jesper_008.SM_Jesper_008"))
    (:9
      (Components|StaticMesh|SetStaticMesh _gemstone "/Game/FantasticGems/Meshes/SM_Jesper_009.SM_Jesper_009"))
    (:10
      (Components|StaticMesh|SetStaticMesh _gemstone "/Game/FantasticGems/Meshes/SM_Jesper_010.SM_Jesper_010"))))