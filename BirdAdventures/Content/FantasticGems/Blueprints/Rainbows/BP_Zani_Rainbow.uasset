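; BP_Zani_Rainbow is a gemstone actor that animates rainbow hue shifts on a Zani gem mesh.
; The construction script uses Seed to choose among numbered Zani mesh variants.
; On BeginPlay, it creates a dynamic material instance from the gem's first material slot.
; A timeline, with play rate set by RainbowSpeed, drives that material's center and rim hue parameters through separate tracks.
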(event EventBeginPlay
  (bind _gemstone (Variables|Default|GetGemstone))
  (Components|Timeline|SetPlayRate (Variables|Default|GetRainbow_Timeline) (Variables|Default|GetRainbow%20Speed))
  (bind _returnvalue (Rendering|Material|CreateDynamicMaterialInstance _gemstone 0 (Rendering|Material|GetMaterial _gemstone 0) :!class /Script/Engine.PrimitiveComponent))
  (bind (_direction _hue _hue2) (Timeline|Rainbow_Timeline Play)
    (:Update
      (Rendering|Material|SetScalarParameterValue _returnvalue "Hue Center" _hue :!class /Script/Engine.MaterialInstanceDynamic)
      (Rendering|Material|SetScalarParameterValue _returnvalue "Hue Rim" _hue2 :!class /Script/Engine.MaterialInstanceDynamic))))

(fn ConstructionScript
  (bind _gemstone (Variables|Default|GetGemstone))
  (switch int (Variables|Default|GetSeed)
    (:2
      (Components|StaticMesh|SetStaticMesh _gemstone "/Game/FantasticGems/Meshes/SM_Zani_002.SM_Zani_002"))
    (:3
      (Components|StaticMesh|SetStaticMesh _gemstone "/Game/FantasticGems/Meshes/SM_Zani_003.SM_Zani_003"))
    (:4
      (Components|StaticMesh|SetStaticMesh _gemstone "/Game/FantasticGems/Meshes/SM_Zani_004.SM_Zani_004"))
    (:5
      (Components|StaticMesh|SetStaticMesh _gemstone "/Game/FantasticGems/Meshes/SM_Zani_005.SM_Zani_005"))
    (:6
      (Components|StaticMesh|SetStaticMesh _gemstone "/Game/FantasticGems/Meshes/SM_Zani_006.SM_Zani_006"))
    (:7
      (Components|StaticMesh|SetStaticMesh _gemstone "/Game/FantasticGems/Meshes/SM_Zani_007.SM_Zani_007"))
    (:8
      (Components|StaticMesh|SetStaticMesh _gemstone "/Game/FantasticGems/Meshes/SM_Zani_008.SM_Zani_008"))
    (:9
      (Components|StaticMesh|SetStaticMesh _gemstone "/Game/FantasticGems/Meshes/SM_Zani_009.SM_Zani_009"))
    (:10
      (Components|StaticMesh|SetStaticMesh _gemstone "/Game/FantasticGems/Meshes/SM_Zani_010.SM_Zani_010"))))