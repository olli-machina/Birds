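; Configurable "Spawn" gemstone prop from FantasticGems, set up entirely in the Construction Script with no active runtime logic.
; FreestyleOrPreset either swaps the Gemstone mesh to one of ten presets or, in Freestyle, creates dynamic material instances on its three slots: seed, membrane and rays.
; Exposed variables drive their colors, fresnel, opacity, pulse and world position offset animation, and PickFXColor selects one of six ray FX textures.
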(event EventBeginPlay)

(event Collision|EventActorBeginOverlap
  (params (OtherActor :type Actor%20Object%20Reference)))

(event EventTick
  (params (DeltaSeconds :type Float%20%28single-precision%29)))

(fn ConstructionScript
  (bind _gemstone (Variables|Default|GetGemstone))
  (bind _gemstone_2 (Variables|Default|GetGemstone))
  (switch Utilities|FlowControl|Switch|SwitchonENUM_Demon_Eye_001 (Variables|Control|GetFreestyle%20or%20Preset)
    (:NewEnumerator0
      (bind _returnvalue (Rendering|Material|CreateDynamicMaterialInstance _gemstone 0 (Rendering|Material|GetMaterial _gemstone 0) :!class /Script/Engine.PrimitiveComponent))
      (Rendering|Material|SetScalarParameterValue _returnvalue "Fresnel Power 1" (Variables|Seed|GetSeed%20External%20Fresnel%20Power) :!class /Script/Engine.MaterialInstanceDynamic)
      (Rendering|Material|SetScalarParameterValue _returnvalue "Fresnel Power 2" (Variables|Seed|GetSeed%20Internal%20Fresnel%20Power) :!class /Script/Engine.MaterialInstanceDynamic)
      (Rendering|Material|SetScalarParameterValue _returnvalue "Pulse Speed" (Variables|Seed|GetSeed%20Pulse%20Speed) :!class /Script/Engine.MaterialInstanceDynamic)
      (Rendering|Material|SetScalarParameterValue _returnvalue "Use Pulse" (Variables|Seed|GetSeed%20Pulse%20amount) :!class /Script/Engine.MaterialInstanceDynamic)
      (Rendering|Material|SetVectorParameterValue _returnvalue "Color 1" (Variables|Seed|GetSeed%20Color) :!class /Script/Engine.MaterialInstanceDynamic)
      (bind _returnvalue_2 (Rendering|Material|CreateDynamicMaterialInstance _gemstone 1 "/Game/FantasticGems/Materials/Master/MAT_Spawn_Membrane.MAT_Spawn_Membrane" :!class /Script/Engine.PrimitiveComponent))
      (Rendering|Material|SetVectorParameterValue _returnvalue_2 "Color 1" (Variables|Membrane|GetMembrane%20Color) :!class /Script/Engine.MaterialInstanceDynamic)
      (Rendering|Material|SetScalarParameterValue _returnvalue_2 "Opacity MIN" (Variables|Membrane|GetMembrane%20Opacity%20MIN) :!class /Script/Engine.MaterialInstanceDynamic)
      (Rendering|Material|SetScalarParameterValue _returnvalue_2 "Opacity MAX" (Variables|Membrane|GetMembrane%20Opacity%20MAX) :!class /Script/Engine.MaterialInstanceDynamic)
      (Rendering|Material|SetScalarParameterValue _returnvalue_2 "Fresnel Power 1" (Variables|Membrane|GetMembrane%20Fresnel) :!class /Script/Engine.MaterialInstanceDynamic)
      (Rendering|Material|SetScalarParameterValue _returnvalue_2 "Time Multiply" (Variables|Membrane|GetMembrane%20Pulse%20Speed) :!class /Script/Engine.MaterialInstanceDynamic)
      (Rendering|Material|SetScalarParameterValue _returnvalue_2 "Use Pulse" (Variables|Membrane|Getmembrane%20Pulse%20Amount) :!class /Script/Engine.MaterialInstanceDynamic)
      (Rendering|Material|SetScalarParameterValue _returnvalue_2 "Fresnel Power 2" (Variables|Membrane|GetMembrane%20second%20fresnel) :!class /Script/Engine.MaterialInstanceDynamic)
      (bind _returnvalue_3 (Rendering|Material|CreateDynamicMaterialInstance _gemstone 2 "/Game/FantasticGems/Materials/Master/MAT_Spawn_Lines.MAT_Spawn_Lines" :!class /Script/Engine.PrimitiveComponent))
      (Rendering|Material|SetVectorParameterValue _returnvalue_3 "Color 1" (Variables|Rays|GetRay%20Internal%20Color) :!class /Script/Engine.MaterialInstanceDynamic)
      (Rendering|Material|SetVectorParameterValue _returnvalue_3 "Color 2" (Variables|Rays|GetRay%20External%20Color) :!class /Script/Engine.MaterialInstanceDynamic)
      (Rendering|Material|SetScalarParameterValue _returnvalue_3 "Color Contrast" (Variables|Rays|GetRay%20Contrast%20between%20colors) :!class /Script/Engine.MaterialInstanceDynamic)
      (Rendering|Material|SetScalarParameterValue _returnvalue_3 "Opacity Speed 1" (Variables|Rays|GetRay%20Opacity%20speed%20X) :!class /Script/Engine.MaterialInstanceDynamic)
      (Rendering|Material|SetScalarParameterValue _returnvalue_3 "Opacity Speed 2" (Variables|Rays|GetRay%20Opacity%20Speed%20Y) :!class /Script/Engine.MaterialInstanceDynamic)
      (Rendering|Material|SetScalarParameterValue _returnvalue_3 "WPO Speed 1" (Variables|Rays|GetRay%20WPO%20Speed%201) :!class /Script/Engine.MaterialInstanceDynamic)
      (Rendering|Material|SetScalarParameterValue _returnvalue_3 "WPO Speed 2" (Variables|Rays|GetRay%20WPO%20Speed%202) :!class /Script/Engine.MaterialInstanceDynamic)
      (Rendering|Material|SetScalarParameterValue _returnvalue_3 "WPO Speed 3" (Variables|Rays|GetRay%20WPO%20Speed%203) :!class /Script/Engine.MaterialInstanceDynamic)
      (Rendering|Material|SetScalarParameterValue _returnvalue_3 "WPO Speed 4" (Variables|Rays|GetRay%20WPO%20Speed%204) :!class /Script/Engine.MaterialInstanceDynamic)
      (Rendering|Material|SetScalarParameterValue _returnvalue_3 "Time Multiplier" (Variables|Rays|GetRay%20Pulse%20Speed) :!class /Script/Engine.MaterialInstanceDynamic)
      (Rendering|Material|SetScalarParameterValue _returnvalue_3 "Use Pulse" (Variables|Rays|GetRay%20Pulse%20Amount) :!class /Script/Engine.MaterialInstanceDynamic)
      (Rendering|Material|SetScalarParameterValue _returnvalue_3 "WPO Intensity" (Variables|Rays|GetRay%20WPO%20Intensity) :!class /Script/Engine.MaterialInstanceDynamic)
      (switch int (Variables|Rays|GetPick%20FX%20Color)
        (:1
          (Rendering|Material|SetTextureParameterValue _returnvalue_3 "FX" "/Game/FantasticGems/Textures/T_Spawn_001_M.T_Spawn_001_M"))
        (:2
          (Rendering|Material|SetTextureParameterValue _returnvalue_3 "FX" "/Game/FantasticGems/Textures/T_Spawn_002_M.T_Spawn_002_M"))
        (:3
          (Rendering|Material|SetTextureParameterValue _returnvalue_3 "FX" "/Game/FantasticGems/Textures/T_Spawn_003_M.T_Spawn_003_M"))
        (:4
          (Rendering|Material|SetTextureParameterValue _returnvalue_3 "FX" "/Game/FantasticGems/Textures/T_Spawn_004_M.T_Spawn_004_M"))
        (:5
          (Rendering|Material|SetTextureParameterValue _returnvalue_3 "FX" "/Game/FantasticGems/Textures/T_Spawn_005_M.T_Spawn_005_M"))
        (:6
          (Rendering|Material|SetTextureParameterValue _returnvalue_3 "FX" "/Game/FantasticGems/Textures/T_Spawn_006_M.T_Spawn_006_M"))))
    (:NewEnumerator1
      (Components|StaticMesh|SetStaticMesh _gemstone_2 "/Game/FantasticGems/Meshes/SM_Spawn_001.SM_Spawn_001"))
    (:NewEnumerator2
      (Components|StaticMesh|SetStaticMesh _gemstone_2 "/Game/FantasticGems/Meshes/SM_Spawn_002.SM_Spawn_002"))
    (:NewEnumerator3
      (Components|StaticMesh|SetStaticMesh _gemstone_2 "/Game/FantasticGems/Meshes/SM_Spawn_003.SM_Spawn_003"))
    (:NewEnumerator4
      (Components|StaticMesh|SetStaticMesh _gemstone_2 "/Game/FantasticGems/Meshes/SM_Spawn_004.SM_Spawn_004"))
    (:NewEnumerator5
      (Components|StaticMesh|SetStaticMesh _gemstone_2 "/Game/FantasticGems/Meshes/SM_Spawn_005.SM_Spawn_005"))
    (:NewEnumerator6
      (Components|StaticMesh|SetStaticMesh _gemstone_2 "/Game/FantasticGems/Meshes/SM_Spawn_006.SM_Spawn_006"))
    (:NewEnumerator7
      (Components|StaticMesh|SetStaticMesh _gemstone_2 "/Game/FantasticGems/Meshes/SM_Spawn_007.SM_Spawn_007"))
    (:NewEnumerator8
      (Components|StaticMesh|SetStaticMesh _gemstone_2 "/Game/FantasticGems/Meshes/SM_Spawn_008.SM_Spawn_008"))
    (:NewEnumerator9
      (Components|StaticMesh|SetStaticMesh _gemstone_2 "/Game/FantasticGems/Meshes/SM_Spawn_009.SM_Spawn_009"))
    (:NewEnumerator10
      (Components|StaticMesh|SetStaticMesh _gemstone_2 "/Game/FantasticGems/Meshes/SM_Spawn_010.SM_Spawn_010"))))