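; BP_Maelstrom is a configurable gemstone actor with a vortex-style look, set up entirely in the construction script with no runtime logic.
; FreestyleOrPreset selects the mode, and both modes create a dynamic material instance on the Gemstone mesh.
; Freestyle picks a vortex mask texture by PickVortexStyle and pushes exposed color, hue, opacity, fresnel and dirt parameters into the material.
; Each preset swaps in its own static mesh and overrides only Hue.
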(event EventBeginPlay)

(event Collision|EventActorBeginOverlap
  (params (OtherActor :type Actor%20Object%20Reference)))

(event EventTick
  (params (DeltaSeconds :type Float%20%28single-precision%29)))

(fn ConstructionScript
  (bind _gemstone (Variables|Default|GetGemstone))
  (bind _gemstone_2 (Variables|Default|GetGemstone))
  (switch Utilities|FlowControl|Switch|SwitchonENUM_Demon_Eye_001 (Variables|Control|GetFreestyle%20or%20Preset)
    (:NewEnumerator0
      (bind _returnvalue (Rendering|Material|CreateDynamicMaterialInstance _gemstone 0 (Rendering|Material|GetMaterial _gemstone 0) :!class /Script/Engine.PrimitiveComponent))
      (switch int (Variables|Control|GetPick%20Vortex%20Style)
        (:1
          _)
        (:2
          (Rendering|Material|SetTextureParameterValue _returnvalue "Masks" "/Game/FantasticGems/Textures/T_Maelstrom_002_S.T_Maelstrom_002_S"))
        (:3
          (Rendering|Material|SetTextureParameterValue _returnvalue "Masks" "/Game/FantasticGems/Textures/T_Maelstrom_003_S.T_Maelstrom_003_S"))
        (:4
          (Rendering|Material|SetTextureParameterValue _returnvalue "Masks" "/Game/FantasticGems/Textures/T_Maelstrom_004_S.T_Maelstrom_004_S"))
        (:5
          (Rendering|Material|SetTextureParameterValue _returnvalue "Masks" "/Game/FantasticGems/Textures/T_Maelstrom_005_S.T_Maelstrom_005_S"))
        (:6
          (Rendering|Material|SetTextureParameterValue _returnvalue "Masks" "/Game/FantasticGems/Textures/T_Maelstrom_006_S.T_Maelstrom_006_S"))
        (:7
          (Rendering|Material|SetTextureParameterValue _returnvalue "Masks" "/Game/FantasticGems/Textures/T_Maelstrom_007_S.T_Maelstrom_007_S"))
        (:8
          (Rendering|Material|SetTextureParameterValue _returnvalue "Masks" "/Game/FantasticGems/Textures/T_Maelstrom_008_S.T_Maelstrom_008_S"))
        (:9
          (Rendering|Material|SetTextureParameterValue _returnvalue "Masks" "/Game/FantasticGems/Textures/T_Maelstrom_009_S.T_Maelstrom_009_S"))
        (:10
          (Rendering|Material|SetTextureParameterValue _returnvalue "Masks" "/Game/FantasticGems/Textures/T_Maelstrom_010_S.T_Maelstrom_010_S")))
      (Rendering|Material|SetScalarParameterValue _returnvalue "Hue" (Variables|Default|GetHue) :!class /Script/Engine.MaterialInstanceDynamic)
      (Rendering|Material|SetScalarParameterValue _returnvalue "Albedo Hue" (Variables|Default|GetAlbedo%20Hue) :!class /Script/Engine.MaterialInstanceDynamic)
      (Rendering|Material|SetScalarParameterValue _returnvalue "Desaturation" (Variables|Default|GetAlbedo%20Desaturation) :!class /Script/Engine.MaterialInstanceDynamic)
      (Rendering|Material|SetScalarParameterValue _returnvalue "Inner Vortex Opacity 1" (Variables|Default|GetInner%20Vortex%20Opacity%201) :!class /Script/Engine.MaterialInstanceDynamic)
      (Rendering|Material|SetScalarParameterValue _returnvalue "Inner Vortex Opacity 2" (Variables|Default|GetInner%20Vortex%20Opacity%202) :!class /Script/Engine.MaterialInstanceDynamic)
      (Rendering|Material|SetScalarParameterValue _returnvalue "Inner Vortex Fresnel" (Variables|Default|GetInner%20Vortex%20Gradient) :!class /Script/Engine.MaterialInstanceDynamic)
      (Rendering|Material|SetScalarParameterValue _returnvalue "Outer Vortex Fresnel" (Variables|Default|GetOuter%20Vortex%20Gradient) :!class /Script/Engine.MaterialInstanceDynamic)
      (Rendering|Material|SetScalarParameterValue _returnvalue "Outer Vortex Contrast" (Variables|Default|GetOuter%20Vortex%20Contrast) :!class /Script/Engine.MaterialInstanceDynamic)
      (Rendering|Material|SetScalarParameterValue _returnvalue "Vortex Muddier" (Variables|Default|GetDirt) :!class /Script/Engine.MaterialInstanceDynamic)
      (Rendering|Material|SetVectorParameterValue _returnvalue "Color Add" (Variables|Default|GetAlbedo%20Add) :!class /Script/Engine.MaterialInstanceDynamic)
      (Rendering|Material|SetVectorParameterValue _returnvalue "Internal Eye Color Multiplier" (Variables|Default|GetInternal%20Eye%20Color%20Multiplier) :!class /Script/Engine.MaterialInstanceDynamic)
      (Rendering|Material|SetVectorParameterValue _returnvalue "Out Vortex Color" (Variables|Default|GetOuter%20Vortex%20Color) :!class /Script/Engine.MaterialInstanceDynamic)
      (Rendering|Material|SetVectorParameterValue _returnvalue "Internal Vortex Color 1" (Variables|Default|GetInternal%20Vortex%20Color%201) :!class /Script/Engine.MaterialInstanceDynamic)
      (Rendering|Material|SetVectorParameterValue _returnvalue "Internal Vortex Color 2" (Variables|Default|GetInternal%20Vortex%20Color%202) :!class /Script/Engine.MaterialInstanceDynamic))
    (:NewEnumerator1
      (Components|StaticMesh|SetStaticMesh _gemstone_2 "/Game/FantasticGems/Meshes/SM_Maelstrom_001.SM_Maelstrom_001")
      (bind _returnvalue_2 (Rendering|Material|CreateDynamicMaterialInstance _gemstone_2 0 (Rendering|Material|GetMaterial _gemstone_2 0) :!class /Script/Engine.PrimitiveComponent :!label _label))
      (Rendering|Material|SetScalarParameterValue _returnvalue_2 "Hue" (Variables|Default|GetHue) :!class /Script/Engine.MaterialInstanceDynamic))
    (:NewEnumerator2
      (Components|StaticMesh|SetStaticMesh _gemstone_2 "/Game/FantasticGems/Meshes/SM_Maelstrom_002.SM_Maelstrom_002")
      (goto _label))
    (:NewEnumerator3
      (Components|StaticMesh|SetStaticMesh _gemstone_2 "/Game/FantasticGems/Meshes/SM_Maelstrom_003.SM_Maelstrom_003")
      (goto _label))
    (:NewEnumerator4
      (Components|StaticMesh|SetStaticMesh _gemstone_2 "/Game/FantasticGems/Meshes/SM_Maelstrom_004.SM_Maelstrom_004")
      (goto _label))
    (:NewEnumerator5
      (Components|StaticMesh|SetStaticMesh _gemstone_2 "/Game/FantasticGems/Meshes/SM_Maelstrom_005.SM_Maelstrom_005")
      (goto _label))
    (:NewEnumerator6
      (Components|StaticMesh|SetStaticMesh _gemstone_2 "/Game/FantasticGems/Meshes/SM_Maelstrom_006.SM_Maelstrom_006")
      (goto _label))
    (:NewEnumerator7
      (Components|StaticMesh|SetStaticMesh _gemstone_2 "/Game/FantasticGems/Meshes/SM_Maelstrom_007.SM_Maelstrom_007")
      (goto _label))
    (:NewEnumerator8
      (Components|StaticMesh|SetStaticMesh _gemstone_2 "/Game/FantasticGems/Meshes/SM_Maelstrom_008.SM_Maelstrom_008")
      (goto _label))
    (:NewEnumerator9
      (Components|StaticMesh|SetStaticMesh _gemstone_2 "/Game/FantasticGems/Meshes/SM_Maelstrom_009.SM_Maelstrom_009")
      (goto _label))
    (:NewEnumerator10
      (Components|StaticMesh|SetStaticMesh _gemstone_2 "/Game/FantasticGems/Meshes/SM_Maelstrom_010.SM_Maelstrom_010")
      (goto _label))))