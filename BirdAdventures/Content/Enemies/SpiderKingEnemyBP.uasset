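; Spider king enemy that the player defeats by bonking its head collider.
; Overlapping the actor caches the player, and a head hit from that player spawns a gem, launches the player off and destroys the actor.
; The head hit also clears the IsKing flag on the linked MainEnemy Whispa.
; Contact damage is inactive: the DamageTheHero timer setup is unconnected, though end overlap still clears it.
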(event OnComponentBeginOverlap(HeadCollider)
  (params (OverlappedComponent :type Primitive%20Component%20Object%20Reference) (OtherActor :type Actor%20Object%20Reference) (OtherComp :type Primitive%20Component%20Object%20Reference) (OtherBodyIndex :type Integer) (bFromSweep :type Boolean) (SweepResult :type Hit%20Result%20Structure%20%28by%20ref%29))
  (if (== OtherActor (Variables|Default|GetPlayerBird))
    (Variables|Default|SetBonked true)
    (CallFunction|HitHead)
    (bind _asbp_whispa_d (Utilities|Casting|CastToBP_Whispa_D (Variables|Default|GetMainEnemy)))
    (Variables|/Game/Monsters_Darkness_Pack/Blueprints/BP_Whispa_D.BP_Whispa_D_C|SetIsKing _asbp_whispa_d false)))

(event OnComponentEndOverlap(HeadCollider)
  (params (OverlappedComponent :type Primitive%20Component%20Object%20Reference) (OtherActor :type Actor%20Object%20Reference) (OtherComp :type Primitive%20Component%20Object%20Reference) (OtherBodyIndex :type Integer)))

(event Custom|DropCrystal
  (Game|SpawnActorfromClass "/Game/Gems/GemsBP.GemsBP_C" (Transformation|GetActorTransform) "Undefined" 0 0))

(event Custom|HitHead
  (if (Variables|Default|GetBonked)
    (CallFunction|DropCrystal)
    (Default|LaunchOffHead (Variables|Default|GetPlayerBird))
    (Actor|DestroyActor)))

(event EventBeginPlay)

(event Collision|EventActorBeginOverlap
  (params (OtherActor :type Actor%20Object%20Reference))
  (bind _asplayer_blueprint (Utilities|Casting|CastToPlayer_Blueprint OtherActor))
  (Variables|Default|SetPlayerBird _asplayer_blueprint))

(event EventTick
  (params (DeltaSeconds :type Float%20%28single-precision%29)))

(event Collision|EventActorEndOverlap
  (params (OtherActor :type Actor%20Object%20Reference))
  (if (== OtherActor (Variables|Default|GetPlayerBird))
    (Utilities|Time|ClearTimerbyFunctionName 0 "DamageTheHero")))

(fn ConstructionScript)