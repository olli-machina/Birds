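; Gem actor that launches itself at a referenced Enemy as a thrown projectile.
; Any overlap first calls Throw, which enables physics on the Sphere and adds velocity scaled by Power toward a point above the Enemy's location.
; If the overlapping actor is that Enemy, the gem damages it and destroys itself; otherwise it prints the actor's name.
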(event Custom|Throw
  (bind _sphere (Variables|Default|GetSphere))
  ;[1 1 1] Throw Crystal at Enemy
  (Physics|SetSimulatePhysics _sphere true)
  (Class|PrimitiveComponent|SetAllPhysicsLinearVelocity _sphere (* (Math|Vector|GetUnitDirection(Vector) (.Location (Math|Transform|BreakTransform (Transformation|GetActorTransform))) (+ (.Location (Math|Transform|BreakTransform (Transformation|GetActorTransform (Variables|Default|GetEnemy)))) "0,0.000000,300.000000")) (Variables|Default|GetPower)) true))

(event EventBeginPlay)

(event Collision|EventActorBeginOverlap
  (params (OtherActor :type Actor%20Object%20Reference))
  ;[1 1 1] Destroy gem if hit enemy
  (CallFunction|Throw)
  (if (== (Variables|Default|GetEnemy) OtherActor)
    (Default|TakeDamage (Variables|Default|GetEnemy))
    (Actor|DestroyActor)
    (else
      (Development|PrintString (Utilities|GetDisplayName OtherActor)))))

(event EventTick
  (params (DeltaSeconds :type Float%20%28single-precision%29)))

(fn ConstructionScript)