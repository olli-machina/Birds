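; Whispa monster enemy that attacks the player with a fireball and spawns spider minions, with gem spawning still in progress.
; Three seconds after BeginPlay, or on AttackPlayer, it sets a SendAttack timer, spawns a fireball given the player's location, then a spider given the player reference.
; Rest cancels the timer, and TakeDamage flags the animation Blueprint.
; Spawn positions are hard-coded, SendAttack only prints, and direct animation and force nodes are unwired.
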(event Custom|AttackPlayer
  (bind _returnvalue (Transformation|GetActorRotation))
  (bind _returnvalue_2 (Math|Rotator|GetRotationXVector _returnvalue))
  ;[1 1 1] Attack Player
  (bind _returnvalue_3 (Utilities|Time|SetTimerbyFunctionName 0 "SendAttack" 2.5))
  (bind _output_get (Variables|Default|SetForward (Math|Vector|MakeVector (.x _returnvalue_2) (+ (.y _returnvalue_2) 45.0) (.z _returnvalue_2))))
  (bind _returnvalue_4 (Game|SpawnActorfromClass "/Game/FireballObj_Blueprint.FireballObj_Blueprint_C" (Math|Transform|MakeTransform "272.000000,269.000000,150.000000" (Math|Conversions|RotationFromXVector _output_get)) "Undefined" 0 0))
  (Variables|/Game/FireballObj_Blueprint.FireballObj_Blueprint_C|SetPlayerLoc _returnvalue_4 (Transformation|GetActorLocation (Game|GetPlayerCharacter 0)))
  (CallFunction|SpawnSpider))

(event Custom|Rest
  ;[1 1 1] Attack Player
  (Utilities|Time|ClearandInvalidateTimerbyHandle (stale Custom|AttackPlayer _returnvalue_3))
  (Variables|Default|SetAttack false))

(event Custom|SpawnGem
  ;[1 1 1] Spawn Gem (in progress)
  (Game|SpawnActorfromClass "/Game/Gems/GemsBP.GemsBP_C" (Variables|Default|GetCrystal1Location) "AdjustIfPossibleButAlwaysSpawn" 0 0))

(event Custom|TakeDamage
  (Development|PrintString "Damage")
  (Variables|/Game/Animations/Enemy1BP.Enemy1BP_C|SetIsDamaged (Variables|Default|GetAnimationBP) true))

(event Custom|SpawnSpider
  (bind _returnvalue (Game|SpawnActorfromClass "/Game/Enemies/CuteSpiderEnemyBP.CuteSpiderEnemyBP_C" (Math|Transform|MakeTransform (Math|Vector|MakeVector 469.0 (.y (.Location (Math|Transform|BreakTransform (Math|Transform|MakeTransform "272.000000,269.000000,150.000000" (Math|Conversions|RotationFromXVector (stale Custom|AttackPlayer _output_get)))))) 126.0) (.Rotation (Math|Transform|BreakTransform (Math|Transform|MakeTransform "272.000000,269.000000,150.000000" (Math|Conversions|RotationFromXVector (stale Custom|AttackPlayer _output_get))))) (.Scale (Math|Transform|BreakTransform (Math|Transform|MakeTransform "272.000000,269.000000,150.000000" (Math|Conversions|RotationFromXVector (stale Custom|AttackPlayer _output_get)))))) "Undefined" 0 0))
  (bind _output_get (Variables|/Script/Engine.Pawn|SetAIControllerClass _returnvalue "/Game/Enemies/SpiderEnemyAI.SpiderEnemyAI_C"))
  (bind _asplayer_blueprint (Utilities|Casting|CastToPlayer_Blueprint (Game|GetPlayerCharacter 0)))
  (Variables|/Game/Enemies/CuteSpiderEnemyBP.CuteSpiderEnemyBP_C|SetPlayerBird _returnvalue _asplayer_blueprint)
  (Development|PrintString (Utilities|GetClassDisplayName _output_get)))

(event EventBeginPlay
  (bind _returnvalue (Transformation|GetActorRotation))
  (bind _returnvalue_2 (Math|Rotator|GetRotationXVector _returnvalue))
  (Utilities|FlowControl|Delay 3.0)
  ;[1 1 1] Attack Player
  (bind _returnvalue_3 (Utilities|Time|SetTimerbyFunctionName 0 "SendAttack" 2.5))
  (bind _output_get (Variables|Default|SetForward (Math|Vector|MakeVector (.x _returnvalue_2) (+ (.y _returnvalue_2) 45.0) (.z _returnvalue_2))))
  (bind _returnvalue_4 (Game|SpawnActorfromClass "/Game/FireballObj_Blueprint.FireballObj_Blueprint_C" (Math|Transform|MakeTransform "272.000000,269.000000,150.000000" (Math|Conversions|RotationFromXVector _output_get)) "Undefined" 0 0))
  (Variables|/Game/FireballObj_Blueprint.FireballObj_Blueprint_C|SetPlayerLoc _returnvalue_4 (Transformation|GetActorLocation (Game|GetPlayerCharacter 0)))
  (CallFunction|SpawnSpider))

(event Collision|EventActorBeginOverlap
  (params (OtherActor :type Actor%20Object%20Reference)))

(event EventTick
  (params (DeltaSeconds :type Float%20%28single-precision%29)))

(fn ConstructionScript)

(fn SendAttack
  (Development|PrintString "Fire"))